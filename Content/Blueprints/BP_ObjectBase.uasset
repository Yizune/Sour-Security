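; BP_ObjectBase is a base object Blueprint that references an InteractableComponent and a DistractableComponent.
; Four custom events print debug strings when an interaction or distraction starts or finishes.
; The nodes binding these events to the component dispatchers are not reached from any event, so the handlers are never bound here.
; BeginPlay, Tick, overlap and the construction script are empty.
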(event `self.ReceiveBeginPlay`)

(event `OnInteractionStarted_Event_0`
  (`KismetSystemLibrary.PrintString` "Interaction Started"))

(event `OnInteractionFinished_Event_0`
  (`KismetSystemLibrary.PrintString` "Interaction Finished"))

(event `OnDistractionStarted_Event_0`
  (`KismetSystemLibrary.PrintString` "Distraction Started"))

(event `OnDistractionFinished_Event_0`
  (`KismetSystemLibrary.PrintString` "Distraction Finished"))

(fn `UserConstructionScript`)