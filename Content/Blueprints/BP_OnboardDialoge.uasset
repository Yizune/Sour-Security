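; Onboarding tutorial actor that walks the player through switching camera, possessing a lawnmower, using a distraction, electrocuting a coworker and hiding the ragdoll.
; Each step shows dialogue in WBP_Dialoge, colours the speaker name, and waits on a delegate from the referenced level actor to advance.
; A shared looping timer blinks most current targets' highlight or outline through FlipFlops.
; Missing references print warnings, and overlapping the hidden trigger opens Blockout_LVL_Beta.
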(event `self.ReceiveBeginPlay`
  (bind _introdialoge2 (`self.IntroDialoge2`))
  (bind _introdialoge1 (`self.IntroDialoge1`))
  (bind _camera (`self.Camera`))
  (bind _returnvalue (`|CreateWidget` "/Game/UI/WBP_Dialoge.WBP_Dialoge_C"))
  (bind _output_get (set `self.DialogeWidgetRef` _returnvalue))
  (`UserWidget.AddToViewport` _output_get 0)
  (`self.CheckAllRefs`)
  (`self.PutDialogeOnScreen` _introdialoge1)
  (`KismetSystemLibrary.Delay` (`.Duration_4_12C4231F47A43A78E1E0279112D6FE68` (break `/Game/Data/S_Dialoge` _introdialoge1)))
  (`self.PutDialogeOnScreen` _introdialoge2)
  (`KismetSystemLibrary.Delay` (`.Duration_4_12C4231F47A43A78E1E0279112D6FE68` (break `/Game/Data/S_Dialoge` _introdialoge2)))
  (`/Engine/EditorBlueprintResources/StandardMacros.IsValid` _camera
    (:`Is Valid`
      (add `Pawn.ReceiveControllerChangedDelegate` _camera (delegate `ReceiveControllerChangedDelegate_Event`))
      (`self.PutDialogeOnScreen` (`self.CamDialoge`))
      ;[1 1 1] Make Cam blink
      (bind _returnvalue_2 (`KismetSystemLibrary.K2_SetTimerDelegate` (delegate `ToggleHighlightCam`) 0.6 true true))
      (set `self.BlinkingTimer` _returnvalue_2))
    (:`Is Not Valid`
      (`KismetSystemLibrary.PrintString` "NO CAMERA REF IN ONBOARDING DIALOGE" true true (struct :`R` 1.0 :`B` 0.021061 :`A` 1.0) 20.0))))

(event `ToggleHighlightCam`
  (bind _camera (`self.Camera`))
  ;[1 1 1] Make Cam blink
  (`/Engine/EditorBlueprintResources/StandardMacros.FlipFlop`
    (:`A`
      (`/Game/Prototype/Blueprints/Player/BP_Camera.StartHighlight` _camera))
    (:`B`
      (`/Game/Prototype/Blueprints/Player/BP_Camera.StopHighlight` _camera))))

(event `ReceiveControllerChangedDelegate_Event`
  (params (Pawn :type "Pawn Object Reference") (OldController :type "Controller Object Reference") (NewController :type "Controller Object Reference"))
  ;[1 1 1] Chage camera view
  (if (== NewController (`GameplayStatics.GetPlayerController` 0))
    (`/Engine/EditorBlueprintResources/StandardMacros.DoOnce` false
      (:`Completed`
        (`KismetSystemLibrary.K2_ClearAndInvalidateTimerHandle` (`self.BlinkingTimer`))
        (`self.PutDialogeOnScreen` (`self.PossessDialoge`))
        (add `/Game/Prototype/Blueprints/Player/Robots/BP_RobotParent.OnPossessed` (`self.LawnMower`) (delegate `LawnmowerControlled`))
        (bind _returnvalue (`KismetSystemLibrary.K2_SetTimerDelegate` (delegate `BlinkLawnMower`) 0.6 true true))
        (set `self.BlinkingTimer` _returnvalue)))))

(event `BlinkLawnMower`
  (bind _lawnmower (`self.LawnMower`))
  (`/Engine/EditorBlueprintResources/StandardMacros.Gate` false :!label _label ; Fixes continous blinking bug
    (:`Exit`
      (`/Engine/EditorBlueprintResources/StandardMacros.FlipFlop`
        (:`A`
          (`/Game/Prototype/Blueprints/Player/Robots/BP_RobotParent.StartHighlight` _lawnmower))
        (:`B`
          (`/Game/Prototype/Blueprints/Player/Robots/BP_RobotParent.StopHighlight` _lawnmower))))))

(event `LawnmowerControlled`
  ;[1 1 1] Possess
  (`KismetSystemLibrary.K2_ClearAndInvalidateTimerHandle` (`self.BlinkingTimer`))
  (`self.PutDialogeOnScreen` (`self.DistractDialoge`))
  (add `/Game/Developers/harshistalker/Proto/Core/Objects/OnBoarding/BP_SprinklerPanel_HTmp.DistractedDispatch` (`self.DitractObject`) (delegate `DistratcionUsed`))
  (bind _returnvalue (`KismetSystemLibrary.K2_SetTimerDelegate` (delegate `BlinkDistract`) 0.6 true true))
  (set `self.BlinkingTimer` _returnvalue)
  (goto _label :!via `Close`))

(event `BlinkDistract`
  (bind _ditractobject (`self.DitractObject`))
  (`/Engine/EditorBlueprintResources/StandardMacros.FlipFlop`
    (:`A`
      (`/Game/Prototype/Blueprints/BI_Interactable.ShowOutline` _ditractobject))
    (:`B`
      (`/Game/Prototype/Blueprints/BI_Interactable.HideOutline` _ditractobject))))

(event `DistratcionUsed`
  ;[1 1 1] Distract
  (`KismetSystemLibrary.K2_ClearAndInvalidateTimerHandle` (`self.BlinkingTimer`))
  (`self.PutDialogeOnScreen` (`self.ElectrocuteDialoge`))
  (add `/Game/Core/AI/FirstIteration/NPCs/BP_Coworker.OnElectrocute` (`self.Worker`) (delegate `CoworkerElectucuted`))
  (bind _returnvalue (`KismetSystemLibrary.K2_SetTimerDelegate` (delegate `BlinkElectrocute`) 0.6 true true))
  (set `self.BlinkingTimer` _returnvalue))

(event `BlinkElectrocute`
  (bind _wireselectrocute (`self.WiresElectrocute`))
  (`/Engine/EditorBlueprintResources/StandardMacros.FlipFlop`
    (:`A`
      (`/Game/Prototype/Blueprints/Objects/BP_Outlet1.ShowOutline` _wireselectrocute))
    (:`B`
      (`/Game/Prototype/Blueprints/Objects/BP_Outlet1.HideOutline` _wireselectrocute))))

(event `CoworkerElectucuted`
  ;[1 1 1] Electrocute
  (`KismetSystemLibrary.K2_ClearAndInvalidateTimerHandle` (`self.BlinkingTimer`))
  (`self.PutDialogeOnScreen` (`self.HideRagdolDialoge`))
  (add `/Game/Blueprints/BP_OnboardHiden.HasOverlaped` (`self.HiddenTrigger`) (delegate `EndTutorial`)))

(event `EndTutorial`
  (`GameplayStatics.OpenLevel` "Blockout_LVL_Beta"))

(fn `CheckAllRefs`
  (`/Engine/EditorBlueprintResources/StandardMacros.IsValid` (`self.Camera`)
    (:`Is Valid`
      (`/Engine/EditorBlueprintResources/StandardMacros.IsValid` (`self.LawnMower`)
        (:`Is Valid`
          (`/Engine/EditorBlueprintResources/StandardMacros.IsValid` (`self.DitractObject`)
            (:`Is Valid`
              (`/Engine/EditorBlueprintResources/StandardMacros.IsValid` (`self.WiresElectrocute`)
                (:`Is Valid`
                  (`/Engine/EditorBlueprintResources/StandardMacros.IsValid` (`self.Worker`)
                    (:`Is Valid`
                      (`/Engine/EditorBlueprintResources/StandardMacros.IsValid` (`self.HiddenTrigger`)
                        (:`Is Not Valid`
                          (`KismetSystemLibrary.PrintString` "REF MISSING IN ONBOARDING DIALOGE" true true (struct :`R` 1.0 :`B` 0.021061 :`A` 1.0) 20.0))))
                    (:`Is Not Valid`
                      (`KismetSystemLibrary.PrintString` "REF MISSING IN ONBOARDING DIALOGE" true true (struct :`R` 1.0 :`B` 0.021061 :`A` 1.0) 20.0))))
                (:`Is Not Valid`
                  (`KismetSystemLibrary.PrintString` "REF MISSING IN ONBOARDING DIALOGE" true true (struct :`R` 1.0 :`B` 0.021061 :`A` 1.0) 20.0))))
            (:`Is Not Valid`
              (`KismetSystemLibrary.PrintString` "REF MISSING IN ONBOARDING DIALOGE" true true (struct :`R` 1.0 :`B` 0.021061 :`A` 1.0) 20.0))))
        (:`Is Not Valid`
          (`KismetSystemLibrary.PrintString` "REF MISSING IN ONBOARDING DIALOGE" true true (struct :`R` 1.0 :`B` 0.021061 :`A` 1.0) 20.0))))
    (:`Is Not Valid`
      (`KismetSystemLibrary.PrintString` "REF MISSING IN ONBOARDING DIALOGE" true true (struct :`R` 1.0 :`B` 0.021061 :`A` 1.0) 20.0))))

(fn `ClearDialoge`
  (bind _dialogewidgetref (`self.DialogeWidgetRef`))
  (`/Game/UI/WBP_Dialoge.UpdateText` _dialogewidgetref "")
  (`/Game/UI/WBP_Dialoge.UpdateName` _dialogewidgetref ""))

(fn `PutDialogeOnScreen`
  (params (Dialoge :type "/Game/Data/S_Dialoge Structure"))
  (bind (_personspeeking _duration _text) (break `/Game/Data/S_Dialoge` Dialoge))
  (bind _dialogewidgetref (`self.DialogeWidgetRef`))
  (`/Game/UI/WBP_Dialoge.UpdateText` _dialogewidgetref _text)
  (`/Game/UI/WBP_Dialoge.UpdateName` _dialogewidgetref (`KismetTextLibrary.Conv_StringToText` (`|GetEnumeratorNameAsString` _personspeeking)))
  (if (`|EnumEquality` _personspeeking "NewEnumerator1")
    (`/Game/UI/WBP_Dialoge.UpdateNameColor` _dialogewidgetref (make `SlateColor` (struct :`R` 0.722917 :`G` 0.103919 :`B` 0.103919 :`A` 1.0)))
    (else
      (`/Game/UI/WBP_Dialoge.UpdateNameColor` _dialogewidgetref (make `SlateColor` (struct :`G` 0.627755 :`B` 0.722917 :`A` 1.0))))))

(fn `UserConstructionScript`)