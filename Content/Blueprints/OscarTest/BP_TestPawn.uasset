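; BP_TestPawn is a test pawn that switches between mouse-look camera control and a free visible cursor.
; IA_ToggleFocus flip-flops Isfocus; switching it off hides the cursor, recenters it and restores game-only input.
; While Isfocus is false, IA_Look applies pitch and yaw and keeps recentering the mouse in the viewport.
; While Isfocus is true, IA_Look only shows the cursor, leaving the camera still.
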(event `EnhancedInput|/Game/ThirdPerson/Input/Actions/IA_Look`
  (params (ActionValue :type "Vector2D Structure") (ElapsedSeconds :type "Float (double-precision)") (TriggeredSeconds :type "Float (double-precision)") (InputAction :type "InputAction Object Reference" :default "/Game/ThirdPerson/Input/Actions/IA_Look.IA_Look"))
  (bind (_returnvalue_x _returnvalue_y) (`KismetMathLibrary.BreakVector2D` (`WidgetLayoutLibrary.GetViewportSize`)))
  (bind _returnvalue (`GameplayStatics.GetPlayerController` 0))
  (:`Triggered`
    (if (not (`self.Isfocus`))
      ;[1 1 1] makes camera follow mouse movements
      (`WidgetBlueprintLibrary.SetInputMode_GameOnly` _returnvalue)
      (`self.AddControllerPitchInput` ActionValue_Y)
      (`self.AddControllerYawInput` ActionValue_X)
      (`PlayerController.SetMouseLocation` _returnvalue (`KismetMathLibrary.FTrunc` (/ _returnvalue_x 2.0)) (`KismetMathLibrary.FTrunc` (/ _returnvalue_y 2.0)))
      (else
        ;[1 1 1] shows mouse cursor
        (set `PlayerController.bShowMouseCursor` true _returnvalue)))))

(event `EnhancedInput|/Game/ThirdPerson/Input/Actions/IA_ToggleFocus`
  (params (ActionValue :type Boolean) (ElapsedSeconds :type "Float (double-precision)") (TriggeredSeconds :type "Float (double-precision)") (InputAction :type "InputAction Object Reference" :default "/Game/ThirdPerson/Input/Actions/IA_ToggleFocus.IA_ToggleFocus"))
  (bind (_returnvalue_x _returnvalue_y) (`KismetMathLibrary.BreakVector2D` (`WidgetLayoutLibrary.GetViewportSize`)))
  (bind _returnvalue (`GameplayStatics.GetPlayerController` 0))
  (:`Started`
    (`/Engine/EditorBlueprintResources/StandardMacros.FlipFlop`
      (:`A`
        (set `self.Isfocus` true))
      (:`B`
        ;[1 1 1] makes mouse focus the camera and resets position to center.
        (set `self.Isfocus` false)
        (set `PlayerController.bShowMouseCursor` false _returnvalue)
        (`PlayerController.SetMouseLocation` _returnvalue (`KismetMathLibrary.FTrunc` (/ _returnvalue_x 2.0)) (`KismetMathLibrary.FTrunc` (/ _returnvalue_y 2.0)))
        (`WidgetBlueprintLibrary.SetInputMode_GameOnly` _returnvalue)))))

(fn `UserConstructionScript`)