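; BP_OnboardTrigger is a trigger actor that reports while a specific Worker actor is inside either of its two box volumes.
; On overlap begin from the Worker, either box restarts a shared looping half-second timer that calls the HasOverlaped dispatcher.
; On overlap end from either box, that timer is cleared, so leaving one box stops the signal even if the Worker remains in the other.
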(event `self.Box.OnComponentBeginOverlap`
  (params (OverlappedComponent :type "PrimitiveComponent Object Reference") (OtherActor :type "Actor Object Reference") (OtherComp :type "PrimitiveComponent Object Reference") (OtherBodyIndex :type Integer) (bFromSweep :type Boolean) (SweepResult :type "HitResult Structure (by ref)"))
  (if (== (`self.Worker`) OtherActor)
    (`KismetSystemLibrary.K2_ClearAndInvalidateTimerHandle` (`self.Timer`))
    (bind _returnvalue (`KismetSystemLibrary.K2_SetTimerDelegate` (delegate `IsInTrigger`) 0.5 true true))
    (set `self.Timer` _returnvalue)))

(event `IsInTrigger`
  (`self.HasOverlaped`))

(event `self.Box1.OnComponentBeginOverlap`
  (params (OverlappedComponent :type "PrimitiveComponent Object Reference") (OtherActor :type "Actor Object Reference") (OtherComp :type "PrimitiveComponent Object Reference") (OtherBodyIndex :type Integer) (bFromSweep :type Boolean) (SweepResult :type "HitResult Structure (by ref)"))
  (if (== (`self.Worker`) OtherActor)
    (`KismetSystemLibrary.K2_ClearAndInvalidateTimerHandle` (`self.Timer`))
    (bind _returnvalue (`KismetSystemLibrary.K2_SetTimerDelegate` (delegate `IsInTrigger`) 0.5 true true))
    (set `self.Timer` _returnvalue)))

(event `self.Box1.OnComponentEndOverlap`
  (params (OverlappedComponent :type "PrimitiveComponent Object Reference") (OtherActor :type "Actor Object Reference") (OtherComp :type "PrimitiveComponent Object Reference") (OtherBodyIndex :type Integer))
  (if (== (`self.Worker`) OtherActor)
    (`KismetSystemLibrary.K2_ClearAndInvalidateTimerHandle` (`self.Timer`))))

(event `self.Box.OnComponentEndOverlap`
  (params (OverlappedComponent :type "PrimitiveComponent Object Reference") (OtherActor :type "Actor Object Reference") (OtherComp :type "PrimitiveComponent Object Reference") (OtherBodyIndex :type Integer))
  (if (== (`self.Worker`) OtherActor)
    (`KismetSystemLibrary.K2_ClearAndInvalidateTimerHandle` (`self.Timer`))))

(fn `UserConstructionScript`)