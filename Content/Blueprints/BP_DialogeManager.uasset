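; Dialogue manager that plays timed dialogue for one task and chains to the next manager.
; The camera's point-of-interest event starts the intro lines; TaskComplete starts the end lines and immediately sets up NextDialogeManager.
; StartDialoge recursively steps through line structs with delays, updating its widget and showing color-coded talk bubbles on NPCs matching the speaker.
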(event `DeactivateBubble`
  (bind _activatednpcsref (`self.ActivatedNPCsRef`))
  ;[1 1 1] hides all of the activated bubbles and then clears list to avoid memory leak or someting
  (for _array_element _activatednpcsref
    (`/Game/UI/WBP_TalkBubble.HideBubble` (`/Game/Prototype/Blueprints/Characters/BP_ThirdPersonCharacter.TalkBubbleRef` _array_element)))
  (`KismetArrayLibrary.Array_Clear` _activatednpcsref))

(event `ActivateBubbles`
  (params (NewParam :type "/Game/Data/E_DialogeNames Enum" :default "NewEnumerator0"))
  ;[1 1 1] looks at all npcs and shows bubble of the ones with same name and also saves refrence
  (for _array_element (`self.Out Actors`)
    (if (`|EnumEquality` NewParam (`/Game/Prototype/Blueprints/Characters/BP_ThirdPersonCharacter.NPCName` _array_element))
      (`KismetArrayLibrary.Array_Add` (`self.ActivatedNPCsRef`) _array_element)
      (`/Game/UI/WBP_TalkBubble.ShowBubble` (`/Game/Prototype/Blueprints/Characters/BP_ThirdPersonCharacter.TalkBubbleRef` _array_element) (`KismetMathLibrary.Conv_LinearColorToColor` (`.SpecifiedColor` (break `SlateColor` (`BlueprintMapLibrary.Map_Find` (`self.TextColor`) NewParam))))))))

(event `self.ReceiveBeginPlay`
  (`/Engine/EditorBlueprintResources/StandardMacros.IsValid` (`self.NextDialogeManager`)
    (:`Is Valid`
      _)
    (:`Is Not Valid`
      (`KismetSystemLibrary.PrintString` (`KismetStringLibrary.Concat_StrStr` "NO dialoge manager after " (`KismetSystemLibrary.GetDisplayName` self)))))
  (bind _returnvalue (`|CreateWidget` "/Game/UI/WBP_Dialoge.WBP_Dialoge_C"))
  (`UserWidget.AddToViewport` _returnvalue 0)
  (set `self.DialogeWidgetRef` _returnvalue)
  (`self.ClearText`)
  ;[1 1 1] Get all NPC characters
  (bind _outactors (`GameplayStatics.GetAllActorsOfClass` "/Game/Prototype/Blueprints/Characters/BP_ThirdPersonCharacter.BP_ThirdPersonCharacter_C"))
  (set `self.Out Actors` _outactors)
  (if (`self.StartOnBeginPlay?`)
    (`KismetSystemLibrary.Delay` 2.0)
    (`self.SetUpCurrentCamera`)))

(event `SetUpCurrentCamera`
  (bind _startdialogecamera (`self.StartDialogeCamera`))
  ;[1 1 1] Sets up everything for once the camarea has been possesed
  (add `/Game/Prototype/Blueprints/Player/BP_Camera.PlayerHasGoneToIntrest` _startdialogecamera (delegate `PlayerHasGoneToIntrest`))
  (`/Game/Prototype/Blueprints/Player/BP_Camera.ShowIntrestIcon` _startdialogecamera))

(event `PlayerHasGoneToIntrest`
  ;[1 1 1] Sets up everything for once the camarea has been possesed
  (`self.StartDialoge` (`self.DialogeStartTask`)))

(event `StartDialoge`
  (params (DialogeToPlay :type "Array of /Game/Data/S_Dialoge Structure"))
  (bind _index (`self.Index`))
  (bind _dialogewidgetref (`self.DialogeWidgetRef`))
  (bind (_personspeeking _duration _text) (break `/Game/Data/S_Dialoge` (`|GetArrayItem` DialogeToPlay _index)))
  ;[1 1 1] Dialoge system. handles all of the funtionality for takeing in structs and outputting text and dialoge boxes.
  (if (not (>= _index (`KismetArrayLibrary.Array_Length` DialogeToPlay)))
    (if (not (`|EnumEquality` _personspeeking "NewEnumerator0"))
      (`/Game/UI/WBP_Dialoge.UpdateText` _dialogewidgetref _text)
      (`/Game/UI/WBP_Dialoge.UpdateName` _dialogewidgetref (`KismetTextLibrary.Conv_StringToText` (`KismetStringLibrary.Concat_StrStr` (`|GetEnumeratorNameAsString` _personspeeking) " : ")))
      (`self.ActivateBubbles` _personspeeking)
      (`/Game/UI/WBP_Dialoge.UpdateNameColor` _dialogewidgetref (`BlueprintMapLibrary.Map_Find` (`self.TextColor`) _personspeeking))
      (`KismetSystemLibrary.Delay` _duration)
      (`/Engine/EditorBlueprintResources/StandardMacros.IncrementInt` (`self.Index`)
        (:`  `
          (`self.DeactivateBubble`)
          (`self.StartDialoge` DialogeToPlay) ; Loops
        ))
      (else
        (`/Engine/EditorBlueprintResources/StandardMacros.IncrementInt` (`self.Index`)
          (:`  `
            (`self.StartDialoge` DialogeToPlay) ; Loops
          ))))
    (else
      (`self.ClearText`))))

(event `TaskComplete`
  (bind _nextdialogemanager (`self.NextDialogeManager`))
  (`self.StartDialoge` (`self.DialogeEndTask`))
  (`/Engine/EditorBlueprintResources/StandardMacros.IsValid` _nextdialogemanager
    (:`Is Valid`
      (`self.SetUpCurrentCamera` _nextdialogemanager))))

(fn `ClearText`
  (`/Game/UI/WBP_Dialoge.UpdateText` (`self.DialogeWidgetRef`) "")
  (`/Game/UI/WBP_Dialoge.UpdateName` (`self.DialogeWidgetRef`) ""))

(fn `UserConstructionScript`)