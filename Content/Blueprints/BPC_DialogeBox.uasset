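; BPC_DialogeBox is a Blueprint that shows a timed sequence of dialogue lines through a WBP_Dialoge widget.
; BeginPlay creates the widget, keeps a reference and clears its text, with no viewport add in this graph.
; StartDialoge loops through DialogeList by Index, setting each entry's text and waiting its Duration before advancing.
; The loop has no end or bounds check.
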(event `self.ReceiveBeginPlay`
  (bind _returnvalue (`|CreateWidget` "/Game/UI/WBP_Dialoge.WBP_Dialoge_C"))
  (bind _output_get (set `self.DialogeWidgetRef` _returnvalue))
  (`/Game/UI/WBP_Dialoge.UpdateText` _output_get ""))

(event `StartDialoge`
  (bind (_personspeeking _duration _text) (break `/Game/Data/S_Dialoge` (`|GetArrayItem` (`self.DialogeList`) (`self.Index`))))
  (`/Game/UI/WBP_Dialoge.UpdateText` (`self.DialogeWidgetRef`) _text :!label _label)
  (`KismetSystemLibrary.Delay` _duration)
  (set `self.Index` (+ (`self.Index`) 1))
  (goto _label))