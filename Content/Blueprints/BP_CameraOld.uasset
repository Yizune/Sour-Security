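; BP_CameraOld is a possessable camera pawn that lets the player hop to another camera of the same class.
; While possessed, it sphere-traces forward and right each tick to cache neighbouring cameras, with debug drawing on.
; W possesses the cached forward camera; the right one is stored but unused here.
; Mouse look runs through a gate that, when UseFocus is set, the focus toggle closes to show the cursor.
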(event `self.ReceivePossessed`
  (params (NewController :type "Controller Object Reference"))
  (set `self.IsPossesed?` true))

(event `Key|W`
  (params (Key :type "Key Structure"))
  (bind _returnvalue (`GameplayStatics.GetPlayerController` 0))
  (bind _pawnforward (`self.PawnForward`))
  (:`Pressed`
    (`/Engine/EditorBlueprintResources/StandardMacros.IsValid` _pawnforward
      (:`Is Valid`
        (`Controller.UnPossess` _returnvalue)
        (`Controller.Possess` _returnvalue _pawnforward)))))

(event `self.ReceiveUnpossessed`
  (params (OldController :type "Controller Object Reference"))
  (set `self.IsPossesed?` false))

(event `self.ReceiveTick`
  (params (DeltaSeconds :type "Float (single-precision)"))
  (bind _returnvalue (`self.K2_GetActorLocation`))
  (bind (_returnvalue_roll _returnvalue_pitch _returnvalue_yaw) (`KismetMathLibrary.BreakRotator` (`self.K2_GetActorRotation`)))
  (bind _returnvalue_2 (`self.K2_GetActorLocation`))
  (bind (_returnvalue_roll_2 _returnvalue_pitch_2 _returnvalue_yaw_2) (`KismetMathLibrary.BreakRotator` (`self.K2_GetActorRotation`)))
  (if (`self.IsPossesed?`)
    ;[1 1 1] Forward trace
    (`|ExecutionSequence`
      (:`then_0`
        (bind _outhit (`KismetSystemLibrary.SphereTraceSingle` :`Start` _returnvalue_2 :`End` (+ _returnvalue_2 (* (`KismetMathLibrary.GetForwardVector` (`KismetMathLibrary.MakeRotator` _returnvalue_roll 0.0 _returnvalue_yaw)) 2000.0)) :`Radius` 100.0 :`TraceChannel` "TraceTypeQuery3" :`DrawDebugType` "ForOneFrame"))
        (if (`GameplayStatics.BreakHitResult` _outhit)
          (bind _asbp_camera (cast `/Game/Blueprints/BP_CameraOld` (`.HitActor` (`GameplayStatics.BreakHitResult` _outhit))))
          (set `self.PawnForward` _asbp_camera)))
      (:`then_1`
        (bind _outhit_2 (`KismetSystemLibrary.SphereTraceSingle` :`Start` _returnvalue :`End` (+ _returnvalue (* (`KismetMathLibrary.GetForwardVector` (`KismetMathLibrary.MakeRotator` _returnvalue_roll_2 0.0 (+ _returnvalue_yaw_2 90.0))) 2000.0)) :`Radius` 100.0 :`TraceChannel` "TraceTypeQuery3" :`DrawDebugType` "ForOneFrame"))
        (if (`GameplayStatics.BreakHitResult` _outhit_2)
          (bind _asbp_camera_2 (cast `/Game/Blueprints/BP_CameraOld` (`.HitActor` (`GameplayStatics.BreakHitResult` _outhit_2))))
          (set `self.PawnRight` _asbp_camera_2))))))

(event `self.ReceiveBeginPlay`)

(event `EnhancedInput|/Game/ThirdPerson/Input/Actions/IA_Look`
  (params (ActionValue :type "Vector2D Structure") (ElapsedSeconds :type "Float (double-precision)") (TriggeredSeconds :type "Float (double-precision)") (InputAction :type "InputAction Object Reference" :default "/Game/ThirdPerson/Input/Actions/IA_Look.IA_Look"))
  (bind (_returnvalue_x _returnvalue_y) (`KismetMathLibrary.BreakVector2D` (`WidgetLayoutLibrary.GetViewportSize`)))
  (bind _returnvalue (`GameplayStatics.GetPlayerController` 0))
  (:`Triggered`
    (`|ExecutionSequence`
      (:`then_0`
        (`/Engine/EditorBlueprintResources/StandardMacros.Gate` false :!label _label
          (:`Exit`
            (`self.AddControllerPitchInput` ActionValue_Y)
            (`self.AddControllerYawInput` ActionValue_X))))
      (:`then_1`
        ;[1 1 1] whant to use focus?
        (if (`self.UseFocus`)
          (if (`self.IsInFocus?`)
            ;[1 1 1] shows mouse cursor
            (set `PlayerController.bShowMouseCursor` true _returnvalue)
            (goto _label :!via `Close`)
            (else
              ;[1 1 1] makes camera follow mouse movements
              (`WidgetBlueprintLibrary.SetInputMode_GameOnly` _returnvalue)
              (`PlayerController.SetMouseLocation` _returnvalue (`KismetMathLibrary.FTrunc` (/ _returnvalue_x 2.0)) (`KismetMathLibrary.FTrunc` (/ _returnvalue_y 2.0)))
              (set `PlayerController.bShowMouseCursor` false _returnvalue)
              (goto _label :!via `Open`))))))))

(event `EnhancedInput|/Game/ThirdPerson/Input/Actions/IA_ToggleFocus`
  (params (ActionValue :type Boolean) (ElapsedSeconds :type "Float (double-precision)") (TriggeredSeconds :type "Float (double-precision)") (InputAction :type "InputAction Object Reference" :default "/Game/ThirdPerson/Input/Actions/IA_ToggleFocus.IA_ToggleFocus"))
  (bind (_returnvalue_x _returnvalue_y) (`KismetMathLibrary.BreakVector2D` (`WidgetLayoutLibrary.GetViewportSize`)))
  (bind _returnvalue (`GameplayStatics.GetPlayerController` 0))
  ;[1 1 1] Focus toggle
  (:`Started`
    (`/Engine/EditorBlueprintResources/StandardMacros.FlipFlop`
      (:`A`
        (set `self.IsInFocus?` true))
      (:`B`
        ;;[1 1 1] makes mouse focus the camera and resets position to center.
        (set `self.IsInFocus?` false)
        (set `PlayerController.bShowMouseCursor` false _returnvalue)
        (`PlayerController.SetMouseLocation` _returnvalue (`KismetMathLibrary.FTrunc` (/ _returnvalue_x 2.0)) (`KismetMathLibrary.FTrunc` (/ _returnvalue_y 2.0)))
        (`WidgetBlueprintLibrary.SetInputMode_GameOnly` _returnvalue)))))

(fn `UserConstructionScript`)