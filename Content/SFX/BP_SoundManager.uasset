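; BP_SoundManager is a sound manager that handles a 2D outside sound and line-of-sight occlusion for actor-linked sounds.
; On BeginPlay it spawns the outside sound after a short delay, then prunes SoundsStruct entries with invalid actors.
; AdjustSound traces from the camera to above each actor, restoring volume when it hits that actor and nearly muting it when blocked.
; EnableOutside and DisableOutside toggle the outside sound's volume.
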(event `self.ReceiveBeginPlay`
  (`KismetSystemLibrary.Delay` 0.2)
  (bind _returnvalue (`GameplayStatics.SpawnSound2D` "/Game/SFX/Ambience/Outside.Outside" 1.0 1.0 0.0 null))
  (set `self.Outside` _returnvalue)
  (for _array_element (`self.SoundsStruct`)
    (`/Engine/EditorBlueprintResources/StandardMacros.IsValid` (`.Actor_5_B4FC10E6724DC9BA4341B3BA6036AB96` (break `/Game/SFX/Struct_Sounds` _array_element))
      (:`Is Not Valid`
        (`KismetArrayLibrary.Array_RemoveItem` (`self.SoundsStruct`) _array_element)))))

(event `AdjustSound`
  (params (Camera :type "Actor Object Reference"))
  (for _array_element (`self.SoundsStruct`)
    (bind (_sound _actor) (break `/Game/SFX/Struct_Sounds` _array_element))
    (bind (_outhit _returnvalue) (`KismetSystemLibrary.LineTraceSingle` :`Start` (`self.K2_GetActorLocation` Camera) :`End` (+ (`self.K2_GetActorLocation` _actor) (0.0 0.0 150.0)) :`TraceChannel` "TraceTypeQuery6" :`DrawDebugType` "Persistent"))
    (if _returnvalue
      (if (== (`.HitActor` (`GameplayStatics.BreakHitResult` _outhit)) _actor)
        (`AudioComponent.SetVolumeMultiplier` _sound 1.0)
        (else
          (bind _outattenuationsettings (`AudioComponent.BP_GetAttenuationSettingsToApply` _sound))
          (`AudioComponent.SetVolumeMultiplier` _sound 0.01))))))

(event `EnableOutside`
  (`AudioComponent.SetVolumeMultiplier` (`self.Outside`) 1.0))

(event `DisableOutside`
  (`AudioComponent.SetVolumeMultiplier` (`self.Outside`) 0.0))

(fn `UserConstructionScript`)