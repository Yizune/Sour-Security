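; Player interaction component that finds the interactable in front of a supplied camera and forwards start and stop interact messages to it.
; Tick traces a dedicated channel, then confirms line of sight with a Visibility trace unless the target allows interaction through walls.
; Target changes update HUD hover texts (interact, overload, boobytrap) and outlines, which show only for a controlled BP_Camera owner.
; Initialize fetches the HUD from the game mode after a short delay to avoid a null reference.
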(event `Initialize`
  (params (Camera :type "CameraComponent Object Reference"))
  (set `self.Camera` Camera)
  ;[1 1 1] Delay to prevent errors related to hud = null when the cast node is triggered
  (`KismetSystemLibrary.Delay` 0.5)
  (bind _asbp_third_person_game_mode (cast `/Game/Prototype/ThirdPerson/Blueprints/BP_ThirdPersonGameMode` (`GameplayStatics.GetGameMode`)))
  (set `self.Hud` (`/Game/Prototype/ThirdPerson/Blueprints/BP_ThirdPersonGameMode.HUD` _asbp_third_person_game_mode)))

(event `self.ReceiveTick`
  (params (DeltaSeconds :type "Float (single-precision)"))
  (bind _returnvalue (`SceneComponent.K2_GetComponentLocation` (`self.Camera`)))
  (set `self.TraceEnd` (+ (* (`SceneComponent.GetForwardVector` (`self.Camera`)) (`self.InteractableDistance`)) _returnvalue))
  (set `self.TraceStart` _returnvalue)
  (bind (_outhit _returnvalue_2) (`KismetSystemLibrary.LineTraceSingle` (`self.TraceStart`) (`self.TraceEnd`) "TraceTypeQuery3"))
  (if _returnvalue_2
    (bind (_bblockinghit _binitialoverlap _time _distance _location _impactpoint _normal _impactnormal _physmat _hitactor) (`GameplayStatics.BreakHitResult` _outhit))
    (bind _interactablethroughwalls (message `/Game/Prototype/Blueprints/BI_Interactable.IsInteractableThroughWalls` _hitactor))
    (if _interactablethroughwalls
      (`self.SetCurrentTarget` _hitactor)
      (else
        ;[1 1 1] Checks for blockable objects between target and camera if InteractableThroughWalls is set to false on target
        (bind _outhit_2 (`KismetSystemLibrary.LineTraceSingle` (`self.TraceStart`) (`self.TraceEnd`) "TraceTypeQuery1"))
        (bind (_bblockinghit_2 _binitialoverlap_2 _time_2 _distance_2 _location_2 _impactpoint_2 _normal_2 _impactnormal_2 _physmat_2 _hitactor_2) (`GameplayStatics.BreakHitResult` _outhit_2))
        (if (== _hitactor_2 _hitactor)
          (`self.SetCurrentTarget` _hitactor_2))))
    (else
      (`self.SetCurrentTarget` null))))

(fn `InteractStart`
  (returns (ContinuousInteraction :type Boolean))
  (message `/Game/Prototype/Blueprints/BI_Interactable.InteractStart` (`self.CurrentTarget`) (`self.GetOwner`) "NewEnumerator0" "NewEnumerator0" 0.0)
  (return false))

(fn `InteractStop`
  (message `/Game/Prototype/Blueprints/BI_Interactable.InteractStop` (`self.CurrentTarget`)))