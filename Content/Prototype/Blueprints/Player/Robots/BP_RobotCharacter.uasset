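; Prototype robot character that responds to interaction by clearing the player controller's current moving pawn.
; BeginPlay caches player controller 0 as BP_Controller, and InteractStart sets that controller's CurrentMovingPawn to None.
; The interaction and worker-task query functions are stubs returning empty values, and interaction through walls is disallowed.
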(event `self.ReceiveBeginPlay`
  (bind _asbp_controller (cast `/Game/Prototype/Blueprints/Player/BP_Controller` (`GameplayStatics.GetPlayerController` 0)))
  (set `self.BP Controller` _asbp_controller))

(event `/Game/Prototype/Blueprints/BI_Interactable.InteractStart`
  (params (TriggeringActor :type "Actor Object Reference") (TypeOfInteraction :type "/Game/Prototype/Blueprints/Enum_InteractionType Enum" :default "NewEnumerator0") (SourceOfInteraction :type "/Game/Prototype/Blueprints/Enum_InteractionSource Enum" :default "NewEnumerator1") (OverloadForce :type "Float (double-precision)"))
  (set `/Game/Prototype/Blueprints/Player/BP_Controller.CurrentMovingPawn` null (`self.BP Controller`)))

(fn `GetActivityAnimations`
  (returns (AnimIn :type "AnimSequence Object Reference") (AnimOut :type "AnimSequence Object Reference"))
  (return null null))

(fn `GetForcedNextTask`
  (returns (ForcedNextTask :type "/Game/Developers/harshistalker/Proto/Core/Objects/BP_WorldObject_HTmp Object Reference"))
  (return null))

(fn `GetHoverText`
  (returns (InteractText :type String) (OverloadText :type String) (BoobytrapText :type String))
  (return "" "" ""))

(fn `GetWorkerDestination`
  (returns (Transform :type "Transform Structure"))
  (return))

(fn `IsInteractableThroughWalls`
  (returns (InteractableThroughWalls :type Boolean))
  (return false))

(fn `UserConstructionScript`)