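; Parent Blueprint for player-possessable robots, handling interaction, outline highlighting, speed boost and suction.
; Initialize caches meshes, controller and onboarding manager, binding their events to custom-depth outlines and interaction unlocking.
; An allowed interaction makes the robot the controller's moving pawn; during onboarding a looping timer blinks its outline until then.
; Boost raises walk speed and overlaps pawns, while suction moves its box onto the nearest interactable, which then follows it on Tick.
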(event `BindHighlight`
  (bind _bp_controller (`self.BP Controller`))
  (add `/Game/Prototype/Blueprints/Player/BP_Controller.OnStartHighlight` _bp_controller (delegate `StartHighlight`))
  (add `/Game/Prototype/Blueprints/Player/BP_Controller.OnStopHighlight` _bp_controller (delegate `StopHighlight`))
  (add `/Game/Prototype/Blueprints/Objects/OnBoarding/BP_OnboardingManager.EnableAllInteractions` (`self.OnboardingManager`) (delegate `TurnOnIntractions`)))

(event `/Game/Prototype/Blueprints/BI_Interactable.ShowOutline`
  (`self.StartHighlight`))

(event `TurnOnIntractions`
  (set `self.EnabledInteractions` "NewEnumerator2"))

(event `StopHighlight`
  (bind _staticmesh (`self.StaticMesh`))
  (`/Engine/EditorBlueprintResources/StandardMacros.IsValid` _staticmesh
    (:`Is Valid`
      (`PrimitiveComponent.SetRenderCustomDepth` _staticmesh false)
      (`PrimitiveComponent.SetRenderCustomDepth` (`self.StaticMesh2`) false))))

(event `StartHighlight`
  (bind _staticmesh (`self.StaticMesh`))
  (switch `/Game/Prototype/Blueprints/Objects/Enum_OnboardingChecks` (`self.EnabledInteractions`)
    (:`NewEnumerator1`
      _)
    (:`NewEnumerator2`
      _))
  (`/Engine/EditorBlueprintResources/StandardMacros.IsValid` _staticmesh
    (:`Is Valid`
      (`PrimitiveComponent.SetRenderCustomDepth` _staticmesh true)
      (`PrimitiveComponent.SetRenderCustomDepth` (`self.StaticMesh2`) true)
      (`PrimitiveComponent.SetCustomDepthStencilValue` (`self.StaticMesh2`) 3))))

(event `/Game/Prototype/Blueprints/BI_Interactable.HideOutline`
  (`self.StopHighlight`))

(event `self.ReceiveBeginPlay`)

(event `/Game/Prototype/Blueprints/BI_Interactable.InteractStart`
  (params (TriggeringActor :type "Actor Object Reference") (TypeOfInteraction :type "/Game/Prototype/Blueprints/Enum_InteractionType Enum" :default "NewEnumerator0") (SourceOfInteraction :type "/Game/Prototype/Blueprints/Enum_InteractionSource Enum" :default "NewEnumerator1") (OverloadForce :type "Float (double-precision)"))
  (bind _success (`self.InteractionCheck` TypeOfInteraction))
  (if _success
    (set `/Game/Prototype/Blueprints/Player/BP_Controller.CurrentMovingPawn` self (`self.BP Controller`))
    (`GameplayStatics.PlaySoundAtLocation` (`self.PossessSound`) (`self.K2_GetActorLocation`) (struct) 1.0 1.0 0.0 "/Game/SFX/SoundAttenuationSettigns.SoundAttenuationSettigns" null null null)
    (`self.OnPossessed`)))

(event `StartBoost`
  (set `CharacterMovementComponent.MaxWalkSpeed` (* (`self.DefaultSpeed`) (`self.BoostFactor`)) (`self.CharacterMovement`))
  (set `self.IsBoosting` true)
  (`PrimitiveComponent.SetCollisionResponseToChannel` (`self.CapsuleComponent`) "ECC_Pawn" "ECR_Overlap"))

(event `StopBoost`
  (set `CharacterMovementComponent.MaxWalkSpeed` (`self.DefaultSpeed`) (`self.CharacterMovement`))
  (set `self.IsBoosting` false)
  (`PrimitiveComponent.SetCollisionResponseToChannel` (`self.CapsuleComponent`) "ECC_Pawn" "ECR_Block"))

(event `self.CapsuleComponent.OnComponentBeginOverlap`
  (params (OverlappedComponent :type "PrimitiveComponent Object Reference") (OtherActor :type "Actor Object Reference") (OtherComp :type "PrimitiveComponent Object Reference") (OtherBodyIndex :type Integer) (bFromSweep :type Boolean) (SweepResult :type "HitResult Structure (by ref)")))

(event `self.CapsuleComponent.OnComponentHit`
  (params (HitComponent :type "PrimitiveComponent Object Reference") (OtherActor :type "Actor Object Reference") (OtherComp :type "PrimitiveComponent Object Reference") (NormalImpulse :type "Vector Structure") (Hit :type "HitResult Structure (by ref)")))

(event `/Game/Prototype/Blueprints/BI_Interactable.TriggerBlink`
  (params (Type :type "/Game/Prototype/Blueprints/Objects/Enum_OnboardingChecks Enum" :default "NewEnumerator0") (Index :type Integer))
  (switch `int` (`self.OnboardingIndex`)
    (:`0`
      (`self.TurnOnIntractions`)
      (bind _returnvalue (`KismetSystemLibrary.K2_SetTimerDelegate` (delegate `ToggleBlink`) 0.7 true))
      (set `self.BlinkTimer` _returnvalue)
      (`/Engine/EditorBlueprintResources/StandardMacros.IncrementInt` (`self.OnboardingIndex`)))
    (:`1`
      (set `/Game/Prototype/Blueprints/Player/BP_Controller.WaitingForOnBoardingMovement` true (`self.BP Controller`)))))

(event `ToggleBlink`
  (`/Engine/EditorBlueprintResources/StandardMacros.FlipFlop`
    (:`A`
      (`self.StartHighlight`))
    (:`B`
      (`self.StopHighlight`))))

(event `/Game/Prototype/Blueprints/BI_Interactable.EnableInteraction`
  (params (Type :type "/Game/Prototype/Blueprints/Objects/Enum_OnboardingChecks Enum" :default "NewEnumerator0"))
  (switch `/Game/Prototype/Blueprints/Objects/Enum_OnboardingChecks` Type
    (:`NewEnumerator0`
      (set `self.EnabledInteractions` "NewEnumerator0"))
    (:`NewEnumerator1`
      (`self.TurnOnIntractions` :!label _label))
    (:`NewEnumerator2`
      (goto _label))))

(event `/Game/Prototype/Blueprints/BI_Interactable.ShiftFunction`
  (params (Enable :type Boolean))
  (bind _overlappingactors (`PrimitiveComponent.GetOverlappingActors` (`self.SuctionBox`) null))
  (if Enable
    (set `self.SuctionDistance` 10000.0)
    (if (`KismetArrayLibrary.Array_IsNotEmpty` _overlappingactors)
      (for _array_element _overlappingactors
        (if (`KismetSystemLibrary.DoesImplementInterface` _array_element "/Game/Prototype/Blueprints/BI_Interactable.BI_Interactable_C")
          (bind _returnvalue (`KismetMathLibrary.Vector_Distance` (`self.K2_GetActorLocation` _array_element) (`SceneComponent.K2_GetComponentLocation` (`self.SuctionBox`))))
          (if (< _returnvalue (`self.SuctionDistance`))
            (set `self.SuctionDistance` _returnvalue)
            (set `self.SuckedActor` _array_element))))
      (`SceneComponent.K2_SetWorldLocation` (`self.SuctionBox`) (`self.K2_GetActorLocation` (`self.SuckedActor`)) false false)
      (set `self.IsSucking` true))
    (else
      (set `self.IsSucking` false))))

(event `self.ReceiveTick`
  (params (DeltaSeconds :type "Float (single-precision)"))
  (if (and (`self.IsSucking`) (`KismetSystemLibrary.IsValid` (`self.SuckedActor`)))
    (`self.K2_SetActorLocation` (`self.SuckedActor`) (`SceneComponent.K2_GetComponentLocation` (`self.SuctionBox`)) false false)))

(fn `GetActivityAnimations`
  (returns (AnimIn :type "AnimSequence Object Reference") (AnimOut :type "AnimSequence Object Reference"))
  (return null null))

(fn `GetForcedNextTask`
  (returns (ForcedNextTask :type "/Game/Developers/harshistalker/Proto/Core/Objects/BP_WorldObject_HTmp Object Reference"))
  (return null))

(fn `GetHoverText`
  (returns (InteractText :type String) (OverloadText :type String) (BoobytrapText :type String))
  (return "" "" ""))

(fn `GetWorkerDestination`
  (returns (Transform :type "Transform Structure"))
  (return))

(fn `Initialize`
  (params (StaticMesh :type "StaticMeshComponent Object Reference") (SkeletalMesh :type "SkeletalMeshComponent Object Reference") (StaticMesh2 :type "StaticMeshComponent Object Reference"))
  (set `self.StaticMesh` StaticMesh)
  (set `self.StaticMesh2` StaticMesh2)
  (set `self.SkeletalMesh` SkeletalMesh)
  (bind _asbp_controller (cast `/Game/Prototype/Blueprints/Player/BP_Controller` (`GameplayStatics.GetPlayerController` 0)))
  (set `self.BP Controller` _asbp_controller)
  (set `self.DefaultSpeed` (`CharacterMovementComponent.MaxWalkSpeed` (`self.CharacterMovement`)))
  (bind _returnvalue (`GameplayStatics.GetActorOfClass` "/Game/Prototype/Blueprints/Objects/OnBoarding/BP_OnboardingManager.BP_OnboardingManager_C"))
  (set `self.OnboardingManager` _returnvalue)
  (`self.BindHighlight`)
  (set `self.StartingTransform` (`self.GetTransform`)))

(fn `InteractionCheck`
  (params (TypeOfInteraction :type "/Game/Prototype/Blueprints/Enum_InteractionType Enum" :default "NewEnumerator0"))
  (returns (Success :type Boolean))
  (bind _blinktimer (`self.BlinkTimer`))
  (switch `/Game/Prototype/Blueprints/Objects/Enum_OnboardingChecks` (`self.EnabledInteractions`)
    (:`NewEnumerator1`
      (switch `/Game/Prototype/Blueprints/Enum_InteractionType` TypeOfInteraction
        (:`NewEnumerator0`
          _)
        (:`NewEnumerator1`
          (return false))))
    (:`NewEnumerator2`
      _))
  (if (`KismetSystemLibrary.K2_IsTimerActiveHandle` _blinktimer)
    (`KismetSystemLibrary.K2_ClearAndInvalidateTimerHandle` _blinktimer)
    (`/Game/Prototype/Blueprints/Objects/OnBoarding/BP_OnboardingManager.NextOnboardingEvent` (`self.OnboardingManager`)))
  (return true))

(fn `IsInteractableThroughWalls`
  (returns (InteractableThroughWalls :type Boolean))
  (return false))

(fn `UserConstructionScript`)