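; BP_MapCam is the player's map-view camera, active while possessed, that reveals security or world camera icons and the building interior.
; On BeginPlay it caches every BP_Camera actor in the level.
; Possession shows each camera's map icon and hides the Roof actor and its mesh children; unpossession reverses both.
; The roof toggle sits inside the camera loop, so it only runs when cameras exist.
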(event `self.ReceiveBeginPlay`
  (bind _outactors (`GameplayStatics.GetAllActorsOfClass` "/Game/Prototype/Blueprints/Player/BP_Camera.BP_Camera_C"))
  (set `self.Cameras` _outactors))

(event `self.ReceivePossessed`
  (params (NewController :type "Controller Object Reference"))
  (bind _roof (`self.Roof`))
  (for _array_element (`self.Cameras`)
    (`/Game/Prototype/Blueprints/Player/BP_Camera.ShowMapIcon` _array_element)
    ;[1 1 1] Show and hide roof of building when using map.
    (`/Engine/EditorBlueprintResources/StandardMacros.IsValid` (`self.Roof`)
      (:`Is Valid`
        (`self.SetActorHiddenInGame` _roof true)
        (`SceneComponent.SetVisibility` (`StaticMeshActor.StaticMeshComponent` _roof) false true)))))

(event `self.ReceiveUnpossessed`
  (params (OldController :type "Controller Object Reference"))
  (bind _roof (`self.Roof`))
  (for _array_element (`self.Cameras`)
    ;[1 1 1] Show and hide roof of building when using map.
    (`/Game/Prototype/Blueprints/Player/BP_Camera.HideMapIcon` _array_element)
    (`/Engine/EditorBlueprintResources/StandardMacros.IsValid` (`self.Roof`)
      (:`Is Valid`
        (`self.SetActorHiddenInGame` _roof false)
        (`SceneComponent.SetVisibility` (`StaticMeshActor.StaticMeshComponent` _roof) true true)))))

(fn `UserConstructionScript`)