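; Interactable actor that, judging by its name, drives menu animation by staging a character and a door.
; On InteractStart it sends TargetCharacter a distract message to move to its own location, then after a brief delay triggers TargetDoor.
; The door receives OppositeManager as the triggering actor rather than this actor.
; Hover texts are empty and interaction through walls is disabled.
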(event `/Game/Prototype/Blueprints/BI_Interactable.InteractStart`
  (params (TriggeringActor :type "Actor Object Reference") (TypeOfInteraction :type "/Game/Prototype/Blueprints/Enum_InteractionType Enum" :default "NewEnumerator0"))
  (message `/Game/Prototype/Blueprints/BI_Character.Distract` (`self.TargetCharacter`) true (`self.K2_GetActorLocation`))
  (`KismetSystemLibrary.Delay` 0.2)
  (`/Game/Prototype/Blueprints/BI_Interactable.InteractStart` (`self.TargetDoor`) (`self.OppositeManager`) "NewEnumerator1"))

(fn `GetHoverText`
  (returns (InteractText :type String) (OverloadText :type String) (BoobytrapText :type String))
  (return "" "" ""))

(fn `IsInteractableThroughWalls`
  (returns (InteractableThroughWalls :type Boolean))
  (return false))

(fn `UserConstructionScript`)