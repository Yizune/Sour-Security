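; BP_BodyTrigger_Master is a box trigger that reacts when a BP_Coworker overlaps it, serving both onboarding and target elimination.
; It finds the onboarding and targets managers on BeginPlay.
; TriggerBlink arms a one-shot flag that makes the next overlap advance onboarding; otherwise the coworker goes to the targets manager's EliminationCheck.
; Its interaction and worker-task functions are empty stubs.
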(event `self.ReceiveBeginPlay`
  (bind _returnvalue (`GameplayStatics.GetActorOfClass` "/Game/Prototype/Blueprints/Objects/OnBoarding/BP_OnboardingManager.BP_OnboardingManager_C"))
  (set `self.OnboardingManager` _returnvalue)
  (bind _returnvalue_2 (`GameplayStatics.GetActorOfClass` "/Game/Prototype/Blueprints/BP_TargetsManager.BP_TargetsManager_C"))
  (set `self.TargetManager` _returnvalue_2))

(event `/Game/Prototype/Blueprints/BI_Interactable.TriggerBlink`
  (params (Type :type "/Game/Prototype/Blueprints/Objects/Enum_OnboardingChecks Enum" :default "NewEnumerator0") (Index :type Integer))
  (set `self.OnboardingTrigger` true))

(event `self.Box.OnComponentBeginOverlap`
  (params (OverlappedComponent :type "PrimitiveComponent Object Reference") (OtherActor :type "Actor Object Reference") (OtherComp :type "PrimitiveComponent Object Reference") (OtherBodyIndex :type Integer) (bFromSweep :type Boolean) (SweepResult :type "HitResult Structure (by ref)"))
  (bind _asbp_coworker (cast `/Game/Core/AI/FirstIteration/NPCs/BP_Coworker` OtherActor))
  (`self.TargetsCheck` _asbp_coworker))

(event `TargetsCheck`
  (params (NPC :type "/Game/Core/AI/FirstIteration/NPCs/BP_Coworker Object Reference"))
  (if (`self.OnboardingTrigger`)
    (`/Game/Prototype/Blueprints/Objects/OnBoarding/BP_OnboardingManager.NextOnboardingEvent` (`self.OnboardingManager`))
    (set `self.OnboardingTrigger` false)
    (else
      (`/Game/Prototype/Blueprints/BP_TargetsManager.EliminationCheck` (`self.TargetManager`) NPC))))

(fn `GetActivityAnimations`
  (returns (AnimIn :type "AnimSequence Object Reference") (AnimOut :type "AnimSequence Object Reference"))
  (return null null))

(fn `GetForcedNextTask`
  (returns (ForcedNextTask :type "/Game/Developers/harshistalker/Proto/Core/Objects/BP_WorldObject_HTmp Object Reference"))
  (return null))

(fn `GetHoverText`
  (returns (InteractText :type String) (OverloadText :type String) (BoobytrapText :type String))
  (return "" "" ""))

(fn `GetWorkerDestination`
  (returns (Transform :type "Transform Structure"))
  (return))

(fn `IsInteractableThroughWalls`
  (returns (InteractableThroughWalls :type Boolean))
  (return false))

(fn `UserConstructionScript`)