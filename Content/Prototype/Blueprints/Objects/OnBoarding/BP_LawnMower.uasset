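; Lawn mower prop for onboarding that can be highlighted and have its interactions switched on or off.
; BeginPlay calls the parent and initializes with the skeletal mesh.
; Highlight events toggle custom depth and stencil on its cylinder and cube part meshes, only when interactions are Fully Enabled.
; EnableInteraction sets the Disabled state directly, while both enabled types call TurnOnIntractions.
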(event `self.ReceiveBeginPlay`
  (`parent.ReceiveBeginPlay`)
  (`self.Initialize` null (`self.Mesh`)))

(event `self.StartHighlight`
  (bind _cylinder13 (`self.Cylinder13`))
  ;[1 1 1] Hilight
  (switch `/Game/Prototype/Blueprints/Objects/Enum_OnboardingChecks` (`self.EnabledInteractions`)
    (:`NewEnumerator2`
      (`PrimitiveComponent.SetRenderCustomDepth` _cylinder13 true)
      (`PrimitiveComponent.SetRenderCustomDepth` (`self.Cube1`) true)
      (`PrimitiveComponent.SetRenderCustomDepth` (`self.Cylinder2`) true)
      (`PrimitiveComponent.SetRenderCustomDepth` (`self.Cylinder`) true)
      (`PrimitiveComponent.SetRenderCustomDepth` (`self.Cylinder3`) true)
      (`PrimitiveComponent.SetRenderCustomDepth` (`self.Cylinder1`) true)
      (`PrimitiveComponent.SetCustomDepthStencilValue` _cylinder13 3)
      (`PrimitiveComponent.SetCustomDepthStencilValue` (`self.Cube1`) 3)
      (`PrimitiveComponent.SetCustomDepthStencilValue` (`self.Cylinder2`) 3)
      (`PrimitiveComponent.SetCustomDepthStencilValue` (`self.Cylinder`) 3)
      (`PrimitiveComponent.SetCustomDepthStencilValue` (`self.Cylinder3`) 3)
      (`PrimitiveComponent.SetCustomDepthStencilValue` (`self.Cylinder1`) 3))))

(event `self.StopHighlight`
  ;[1 1 1] Hilight
  (switch `/Game/Prototype/Blueprints/Objects/Enum_OnboardingChecks` (`self.EnabledInteractions`)
    (:`NewEnumerator2`
      (`PrimitiveComponent.SetRenderCustomDepth` (`self.Cylinder13`) false)
      (`PrimitiveComponent.SetRenderCustomDepth` (`self.Cube1`) false)
      (`PrimitiveComponent.SetRenderCustomDepth` (`self.Cylinder2`) false)
      (`PrimitiveComponent.SetRenderCustomDepth` (`self.Cylinder`) false)
      (`PrimitiveComponent.SetRenderCustomDepth` (`self.Cylinder3`) false)
      (`PrimitiveComponent.SetRenderCustomDepth` (`self.Cylinder1`) false))))

(event `/Game/Prototype/Blueprints/BI_Interactable.EnableInteraction`
  (params (Type :type "/Game/Prototype/Blueprints/Objects/Enum_OnboardingChecks Enum" :default "NewEnumerator0"))
  (switch `/Game/Prototype/Blueprints/Objects/Enum_OnboardingChecks` Type
    (:`NewEnumerator0`
      (set `self.EnabledInteractions` "NewEnumerator0"))
    (:`NewEnumerator1`
      (`self.TurnOnIntractions` :!label _label))
    (:`NewEnumerator2`
      (goto _label))))

(fn `UserConstructionScript`
  (`parent.UserConstructionScript`))