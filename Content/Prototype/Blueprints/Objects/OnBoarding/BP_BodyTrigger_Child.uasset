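; An onboarding trigger volume that reports coworkers entering its box to a BP_BodyTrigger_Master.
; On BeginPlay it finds and caches the master with GetActorOfClass, so it relies on one being present in the level.
; Box overlaps are filtered to BP_Coworker and passed to the master's TargetsCheck.
; The interaction-style functions, such as hover text and worker destination, are empty stubs.
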(event `self.ReceiveBeginPlay`
  (bind _returnvalue (`GameplayStatics.GetActorOfClass` "/Game/Prototype/Blueprints/Objects/OnBoarding/BP_BodyTrigger_Master.BP_BodyTrigger_Master_C"))
  (set `self.BP Body Trigger Master` _returnvalue))

(event `self.Box.OnComponentBeginOverlap`
  (params (OverlappedComponent :type "PrimitiveComponent Object Reference") (OtherActor :type "Actor Object Reference") (OtherComp :type "PrimitiveComponent Object Reference") (OtherBodyIndex :type Integer) (bFromSweep :type Boolean) (SweepResult :type "HitResult Structure (by ref)"))
  (bind _asbp_coworker (cast `/Game/Core/AI/FirstIteration/NPCs/BP_Coworker` OtherActor))
  (`/Game/Prototype/Blueprints/Objects/OnBoarding/BP_BodyTrigger_Master.TargetsCheck` (`self.BP Body Trigger Master`) _asbp_coworker))

(fn `GetActivityAnimations`
  (returns (AnimIn :type "AnimSequence Object Reference") (AnimOut :type "AnimSequence Object Reference"))
  (return null null))

(fn `GetForcedNextTask`
  (returns (ForcedNextTask :type "/Game/Developers/harshistalker/Proto/Core/Objects/BP_WorldObject_HTmp Object Reference"))
  (return null))

(fn `GetHoverText`
  (returns (InteractText :type String) (OverloadText :type String) (BoobytrapText :type String))
  (return "" "" ""))

(fn `GetWorkerDestination`
  (returns (Transform :type "Transform Structure"))
  (return))

(fn `IsInteractableThroughWalls`
  (returns (InteractableThroughWalls :type Boolean))
  (return false))

(fn `UserConstructionScript`)