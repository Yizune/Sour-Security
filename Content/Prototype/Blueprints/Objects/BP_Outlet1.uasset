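; Interactable outlet prop with cables that electrocutes wet puddles as an environmental hazard.
; On interaction, it sends a modifier message to actors overlapping its sphere, electrocutes any BP_WetPuddle among them and plays a sound.
; Controller highlight events toggle a custom-depth outline on the cord pile while interactions are enabled.
; For onboarding, a looping timer blinks the outline; first puddle overlap and the following interaction each advance BP_OnboardingManager.
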(event `TurnOnIntractions`
  (set `self.EnabledInteractions` "NewEnumerator2"))

(event `self.ReceiveBeginPlay`
  (bind _cable (`self.Cable`))
  (bind _asbp_controller (cast `/Game/Prototype/Blueprints/Player/BP_Controller` (`GameplayStatics.GetPlayerController` 0)))
  (set `self.BP Controller` _asbp_controller)
  (bind _returnvalue (`GameplayStatics.GetActorOfClass` "/Game/Prototype/Blueprints/Objects/OnBoarding/BP_OnboardingManager.BP_OnboardingManager_C"))
  (set `self.OnboardingManager` _returnvalue)
  (set `CableComponent.bAttachEnd` true _cable)
  (`CableComponent.SetAttachEndTo` _cable (`self.Outlet`) "None" "None")
  (`CableComponent.SetAttachEndTo` (`self.Cable1`) (`self.Outlet2`) "None" "None")
  (`self.BindHighlight`)
  (bind _asbp_controller_2 (cast `/Game/Prototype/Blueprints/Player/BP_Controller` (`GameplayStatics.GetPlayerController` 0)))
  (set `self.BP Controller` _asbp_controller_2)
  (`self.BindHighlight`)
  (add `/Game/Prototype/Blueprints/Objects/OnBoarding/BP_OnboardingManager.EnableAllInteractions` (`self.OnboardingManager`) (delegate `TurnOnIntractions`)))

(event `BindHighlight`
  (bind _bp_controller (`self.BP Controller`))
  (add `/Game/Prototype/Blueprints/Player/BP_Controller.OnStartHighlight` _bp_controller (delegate `StartHighlight`))
  (add `/Game/Prototype/Blueprints/Player/BP_Controller.OnStopHighlight` _bp_controller (delegate `StopHighlight`)))

(event `StartHighlight`
  (bind _sm_prop_cord_pile_01 (`self.SM_Prop_Cord_Pile_01`))
  (switch `/Game/Prototype/Blueprints/Objects/Enum_OnboardingChecks` (`self.EnabledInteractions`)
    (:`NewEnumerator1`
      _)
    (:`NewEnumerator2`
      _))
  (`PrimitiveComponent.SetRenderCustomDepth` _sm_prop_cord_pile_01 true)
  (`PrimitiveComponent.SetCustomDepthStencilValue` _sm_prop_cord_pile_01 5))

(event `StopHighlight`
  (`PrimitiveComponent.SetRenderCustomDepth` (`self.SM_Prop_Cord_Pile_01`) false))

(event `/Game/Prototype/Blueprints/BI_Interactable.InteractStart`
  (params (TriggeringActor :type "Actor Object Reference") (TypeOfInteraction :type "/Game/Prototype/Blueprints/Enum_InteractionType Enum" :default "NewEnumerator0") (SourceOfInteraction :type "/Game/Prototype/Blueprints/Enum_InteractionSource Enum" :default "NewEnumerator1") (OverloadForce :type "Float (double-precision)"))
  (bind _success (`self.InteractionCheck` "NewEnumerator0"))
  (if _success
    (switch `/Game/Prototype/Blueprints/Objects/Enum_OnboardingChecks` (`self.EnabledInteractions`)
      (:`NewEnumerator1`
        _)
      (:`NewEnumerator2`
        _))
    (for _array_element (`PrimitiveComponent.GetOverlappingActors` (`self.Sphere`) null)
      (message `/Game/Developers/harshistalker/Proto/Core/BPI_Modifiers.StackModifier` _array_element "NewEnumerator0")
      (bind _asbp_wet_puddle (cast `/Game/Developers/harshistalker/Proto/Core/Objects/Spawns/BP_WetPuddle` _array_element))
      (`/Game/Developers/harshistalker/Proto/Core/Objects/Spawns/BP_WetPuddle.Electrocute` _asbp_wet_puddle))
    (`GameplayStatics.PlaySoundAtLocation` "/Game/SFX/Objects/Chord/Chord.Chord" (`self.K2_GetActorLocation`) (struct) 1.0 1.0 0.0 "/Game/SFX/SoundAttenuationSettigns.SoundAttenuationSettigns" null null null)))

(event `/Game/Prototype/Blueprints/BI_Interactable.ShowOutline`
  (`self.StartHighlight`))

(event `/Game/Prototype/Blueprints/BI_Interactable.HideOutline`
  (`self.StopHighlight`))

(event `/Game/Prototype/Blueprints/BI_Interactable.TriggerBlink`
  (params (Type :type "/Game/Prototype/Blueprints/Objects/Enum_OnboardingChecks Enum" :default "NewEnumerator0") (Index :type Integer))
  (`self.TurnOnIntractions`)
  (bind _returnvalue (`KismetSystemLibrary.K2_SetTimerDelegate` (delegate `ToggleBlink`) 0.7 true))
  (set `self.BlinkTimer` _returnvalue)
  (set `self.WaitingForOverlap` true))

(event `ToggleBlink`
  (`/Engine/EditorBlueprintResources/StandardMacros.FlipFlop`
    (:`A`
      (`self.StartHighlight`))
    (:`B`
      (`self.StopHighlight`))))

(event `self.Sphere.OnComponentBeginOverlap`
  (params (OverlappedComponent :type "PrimitiveComponent Object Reference") (OtherActor :type "Actor Object Reference") (OtherComp :type "PrimitiveComponent Object Reference") (OtherBodyIndex :type Integer) (bFromSweep :type Boolean) (SweepResult :type "HitResult Structure (by ref)"))
  (if (== (`GameplayStatics.GetObjectClass` OtherActor) "/Game/Developers/harshistalker/Proto/Core/Objects/Spawns/BP_WetPuddle.BP_WetPuddle_C")
    (`/Engine/EditorBlueprintResources/StandardMacros.DoOnce` false
      (:`Completed`
        (`/Game/Prototype/Blueprints/Objects/OnBoarding/BP_OnboardingManager.NextOnboardingEvent` (`self.OnboardingManager`))
        (set `self.WaitingForOverlap` false)
        (set `self.OnboardingIndex` 1)))))

(event `/Game/Prototype/Blueprints/BI_Interactable.EnableInteraction`
  (params (Type :type "/Game/Prototype/Blueprints/Objects/Enum_OnboardingChecks Enum" :default "NewEnumerator0"))
  (switch `/Game/Prototype/Blueprints/Objects/Enum_OnboardingChecks` Type
    (:`NewEnumerator0`
      (set `self.EnabledInteractions` "NewEnumerator0"))
    (:`NewEnumerator1`
      (`self.TurnOnIntractions` :!label _label))
    (:`NewEnumerator2`
      (goto _label))))

(fn `GetActivityAnimations`
  (returns (AnimIn :type "AnimSequence Object Reference") (AnimOut :type "AnimSequence Object Reference"))
  (return null null))

(fn `GetForcedNextTask`
  (returns (ForcedNextTask :type "/Game/Developers/harshistalker/Proto/Core/Objects/BP_WorldObject_HTmp Object Reference"))
  (return null))

(fn `GetHoverText`
  (returns (InteractText :type String) (OverloadText :type String) (BoobytrapText :type String))
  (return "" "" ""))

(fn `GetWorkerDestination`
  (returns (Transform :type "Transform Structure"))
  (return))

(fn `InteractionCheck`
  (params (TypeOfInteraction :type "/Game/Prototype/Blueprints/Enum_InteractionType Enum" :default "NewEnumerator0"))
  (returns (Success :type Boolean))
  (bind _blinktimer (`self.BlinkTimer`))
  (switch `/Game/Prototype/Blueprints/Objects/Enum_OnboardingChecks` (`self.EnabledInteractions`)
    (:`NewEnumerator1`
      (switch `/Game/Prototype/Blueprints/Enum_InteractionType` TypeOfInteraction
        (:`NewEnumerator0`
          _)
        (:`NewEnumerator1`
          (return false))))
    (:`NewEnumerator2`
      _))
  (if (and (`KismetSystemLibrary.K2_IsTimerActiveHandle` _blinktimer) (== (`self.OnboardingIndex`) 1))
    (`KismetSystemLibrary.K2_ClearAndInvalidateTimerHandle` _blinktimer)
    (`/Game/Prototype/Blueprints/Objects/OnBoarding/BP_OnboardingManager.NextOnboardingEvent` (`self.OnboardingManager`)))
  (return true))

(fn `IsInteractableThroughWalls`
  (returns (InteractableThroughWalls :type Boolean))
  (return false))

(fn `UserConstructionScript`
  (`parent.UserConstructionScript`))