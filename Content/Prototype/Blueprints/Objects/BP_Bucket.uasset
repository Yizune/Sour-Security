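; BP_Bucket is a bucket object that tips over the first time it is hit and spills a puddle.
; A DoOnce on the component hit offsets the Anchor using the horizontal impact delta, intended to make the bucket pivot on its edge.
; The bucket rotates 90 degrees around an axis perpendicular to that delta.
; A downward trace from PuddleSpawnPoint then sets where BP_WetPuddle spawns.
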(event `self.Bucket.OnComponentHit`
  (params (HitComponent :type "PrimitiveComponent Object Reference") (OtherActor :type "Actor Object Reference") (OtherComp :type "PrimitiveComponent Object Reference") (NormalImpulse :type "Vector Structure") (Hit :type "HitResult Structure (by ref)"))
  (bind _returnvalue (`SceneComponent.K2_GetComponentLocation` (`self.PuddleSpawnPoint`)))
  (bind (_returnvalue_x _returnvalue_y) (`KismetMathLibrary.BreakVector` (- (`SceneComponent.K2_GetComponentLocation` (`self.Anchor`)) (`.ImpactPoint` (`GameplayStatics.BreakHitResult` Hit)))))
  ;[1 1 1] Adjust anchor point, so that the bucket is rotated on it's edge
  (`/Engine/EditorBlueprintResources/StandardMacros.DoOnce` false
    (:`Completed`
      (`SceneComponent.K2_AddLocalOffset` (`self.Anchor`) (`KismetMathLibrary.MakeVector` _returnvalue_x _returnvalue_y) false false)
      ;[1 1 1] Rotate bucket
      (`SceneComponent.K2_AddLocalRotation` (`self.Bucket`) (`KismetMathLibrary.RotatorFromAxisAndAngle` (`KismetMathLibrary.GreaterGreater_VectorRotator` (`KismetMathLibrary.MakeVector` _returnvalue_x _returnvalue_y) (struct :`Yaw` 90.0)) 90.0) false false)
      ;[1 1 1] Spawn puddle on the ground in front of the tipped over bucket
      (bind _outhit (`KismetSystemLibrary.LineTraceSingle` _returnvalue (- _returnvalue (0.0 0.0 200.0)) "TraceTypeQuery1"))
      (`|SpawnActorFromClass` "/Game/Developers/harshistalker/Proto/Core/Objects/Spawns/BP_WetPuddle.BP_WetPuddle_C" (`KismetMathLibrary.MakeTransform` (`.Location` (`GameplayStatics.BreakHitResult` _outhit))) "Undefined" "MultiplyWithRoot" null null))))

(fn `UserConstructionScript`)