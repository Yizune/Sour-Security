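; BP_SpawnableParent is a base spawnable physics object that can knock whatever it hits into ragdoll.
; Initialize copies the static mesh from a passed component onto its own StaticMesh, then destroys that component.
; AddForce applies a mass-independent impulse to the mesh.
; On hits above a speed threshold, it sends EnableRagdollMessage to the other actor with scaled velocity plus an upward boost.
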(event `self.StaticMesh.OnComponentHit`
  (params (HitComponent :type "PrimitiveComponent Object Reference") (OtherActor :type "Actor Object Reference") (OtherComp :type "PrimitiveComponent Object Reference") (NormalImpulse :type "Vector Structure") (Hit :type "HitResult Structure (by ref)"))
  (bind _returnvalue (`SceneComponent.GetComponentVelocity` (`self.StaticMesh`)))
  (if (> (`KismetMathLibrary.VSize` _returnvalue) 100.0)
    (message `/Game/Prototype/Blueprints/BI_Ragdoll.EnableRagdoll` OtherActor (+ (* _returnvalue 5.0) (0.0 0.0 1000.0)))))

(event `/Game/Prototype/Blueprints/BI_Force.AddForce`
  (params (ForceVector :type "Vector Structure"))
  (`PrimitiveComponent.AddImpulse` (`self.StaticMesh`) ForceVector "None" true))

(fn `Initialize`
  (params (Mesh :type "StaticMeshComponent Object Reference"))
  (`StaticMeshComponent.SetStaticMesh` (`self.StaticMesh`) (`StaticMeshComponent.StaticMesh` Mesh))
  (`ActorComponent.K2_DestroyComponent` Mesh))

(fn `UserConstructionScript`)