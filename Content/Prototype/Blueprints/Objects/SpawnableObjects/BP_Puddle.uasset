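; BP_Puddle is a puddle object that affects the third-person character on contact and can become electrified.
; Its sphere overlap normally passes the puddle's squeak value to the character.
; SetElectrocute flags it as electrified and reveals the spark particles hidden at BeginPlay, after which overlaps instead send the character a ragdoll call with an upward vector.
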(event `self.ReceiveBeginPlay`
  (`SceneComponent.SetVisibility` (`self.P_Sparks`) false false))

(event `self.Sphere1.OnComponentBeginOverlap`
  (params (OverlappedComponent :type "PrimitiveComponent Object Reference") (OtherActor :type "Actor Object Reference") (OtherComp :type "PrimitiveComponent Object Reference") (OtherBodyIndex :type Integer) (bFromSweep :type Boolean) (SweepResult :type "HitResult Structure (by ref)"))
  (bind _asbp_third_person_character (cast `/Game/Prototype/Blueprints/Characters/BP_ThirdPersonCharacter` OtherActor))
  (if (`self.Electrocute`)
    (message `/Game/Prototype/Blueprints/BI_Ragdoll.EnableRagdoll` _asbp_third_person_character (0.0 0.0 500.0))
    (else
      (`/Game/Prototype/Blueprints/Characters/BP_ThirdPersonCharacter.SetSqueak` _asbp_third_person_character (`self.Squeaks`)))))

(event `SetElectrocute`
  (set `self.Electrocute` true)
  (`SceneComponent.SetVisibility` (`self.P_Sparks`) true false))

(fn `UserConstructionScript`)