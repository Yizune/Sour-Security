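; BP_BodyDestroyer is a trigger object that destroys any BP_Coworker overlapping its Box.
; TriggerBlink sets WaitingForOnboardingTrigger on every BP_BodyDestroyer in the level.
; While that flag is set, a coworker's destruction advances BP_OnboardingManager to its next event and clears the flag on all destroyers, so any one can complete the step.
; Its interaction-style functions, such as hover text and worker destination, are empty stubs.
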(event `self.ReceiveBeginPlay`
  (bind _returnvalue (`GameplayStatics.GetActorOfClass` "/Game/Prototype/Blueprints/Objects/OnBoarding/BP_OnboardingManager.BP_OnboardingManager_C"))
  (set `self.OnboardingManager` _returnvalue))

(event `self.Box.OnComponentBeginOverlap`
  (params (OverlappedComponent :type "PrimitiveComponent Object Reference") (OtherActor :type "Actor Object Reference") (OtherComp :type "PrimitiveComponent Object Reference") (OtherBodyIndex :type Integer) (bFromSweep :type Boolean) (SweepResult :type "HitResult Structure (by ref)"))
  (cast `/Game/Core/AI/FirstIteration/NPCs/BP_Coworker` OtherActor)
  (`self.K2_DestroyActor` OtherActor)
  (if (`self.WaitingForOnboardingTrigger`)
    (`/Game/Prototype/Blueprints/Objects/OnBoarding/BP_OnboardingManager.NextOnboardingEvent` (`self.OnboardingManager`))
    (bind _outactors (`GameplayStatics.GetAllActorsOfClass` "BP_BodyDestroyer_C"))
    (for _array_element _outactors
      (set `/Game/Prototype/Blueprints/Objects/BP_BodyDestroyer.WaitingForOnboardingTrigger` false _array_element))))

(event `/Game/Prototype/Blueprints/BI_Interactable.TriggerBlink`
  (params (Type :type "/Game/Prototype/Blueprints/Objects/Enum_OnboardingChecks Enum" :default "NewEnumerator0"))
  (bind _outactors (`GameplayStatics.GetAllActorsOfClass` "BP_BodyDestroyer_C"))
  (for _array_element _outactors
    (set `/Game/Prototype/Blueprints/Objects/BP_BodyDestroyer.WaitingForOnboardingTrigger` true _array_element)))

(fn `GetActivityAnimations`
  (returns (AnimIn :type "AnimSequence Object Reference") (AnimOut :type "AnimSequence Object Reference"))
  (return null null))

(fn `GetForcedNextTask`
  (returns (ForcedNextTask :type "/Game/Developers/harshistalker/Proto/Core/Objects/BP_WorldObject_HTmp Object Reference"))
  (return null))

(fn `GetHoverText`
  (returns (InteractText :type String) (OverloadText :type String) (BoobytrapText :type String))
  (return "" "" ""))

(fn `GetWorkerDestination`
  (returns (Transform :type "Transform Structure"))
  (return))

(fn `IsInteractableThroughWalls`
  (returns (InteractableThroughWalls :type Boolean))
  (return false))

(fn `UserConstructionScript`)