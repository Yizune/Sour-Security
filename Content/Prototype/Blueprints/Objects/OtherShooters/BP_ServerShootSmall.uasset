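; Interactable small server cabinet that distracts characters when the player uses it and ejects server nodes when overloaded.
; Interactions are routed by behaviour enums: Distract sphere-traces for a character to message, while Spawn swaps a random child mesh for a spawned BP_HitSpawn_SmallServerNode.
; Boobytrapping makes NPC use trigger the overload.
; It also handles stencil highlighting and a camera-facing overload bar, and BP_OnboardingManager can fully enable its interactions.
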(event `self.ReceiveBeginPlay`
  (`self.Initialize` 300.0 null "NewEnumerator1" "NewEnumerator5" (`self.SM_Prop_Server_Cabinet_03`) null false null null 20000.0 "/Game/Developers/harshistalker/Proto/Core/Objects/Spawns/BP_HitSpawn_SmallServerNode.BP_HitSpawn_SmallServerNode_C")
  (set `self.MeshArray` (`SceneComponent.GetChildrenComponents` (`self.SM_Prop_Server_Cabinet_03`) false))
  (bind _returnvalue (`|CreateWidget` "/Game/UI/WB_OverloadBar.WB_OverloadBar_C"))
  (`WidgetComponent.SetWidget` (`self.OverloadBar`) _returnvalue)
  (bind _returnvalue_2 (`GameplayStatics.GetActorOfClass` "/Game/Prototype/Blueprints/Objects/OnBoarding/BP_OnboardingManager.BP_OnboardingManager_C"))
  (add `/Game/Prototype/Blueprints/Objects/OnBoarding/BP_OnboardingManager.EnableAllInteractions` _returnvalue_2 (delegate `TurnOnInteractions`)))

(event `TurnOnInteractions`
  (set `self.EnabledInteractions` "NewEnumerator2"))

(event `self.InteractStart`
  (params (TriggeringActor :type "Actor Object Reference") (TypeOfInteraction :type "/Game/Prototype/Blueprints/Enum_InteractionType Enum" :default "NewEnumerator0") (SourceOfInteraction :type "/Game/Prototype/Blueprints/Enum_InteractionSource Enum" :default "NewEnumerator1") (OverloadForce :type "Float (double-precision)"))
  (switch `/Game/Prototype/Blueprints/Objects/Enum_OnboardingChecks` (`self.EnabledInteractions`)
    (:`NewEnumerator1`
      _)
    (:`NewEnumerator2`
      _))
  (set `self.TypeOfInteraction` TypeOfInteraction)
  (set `self.InteractionSource` SourceOfInteraction)
  (set `self.OverloadForce` OverloadForce)
  (switch `/Game/Prototype/Blueprints/Enum_InteractionType` (`self.TypeOfInteraction`)
    (:`NewEnumerator0`
      (if (`self.Boobytrapped`)
        (switch `/Game/Prototype/Blueprints/Enum_InteractionSource` (`self.InteractionSource`)
          (:`NewEnumerator1`
            ;[1 1 1] Trigger overload if boobytrapped and character is interacting
            (message `/Game/Prototype/Blueprints/BI_Interactable.InteractStart` self null "NewEnumerator1" (`self.InteractionSource`) 0.0))
          (:`NewEnumerator0`
            (switch `/Game/Prototype/Blueprints/Enum_InteractionBehaviour` (`self.InteractBehaviour`) :!label _label
              (:`NewEnumerator0`
                (`self.Open/CLose` :!label _label_2))
              (:`NewEnumerator1`
                (`self.Distract` :!label _label_3))
              (:`NewEnumerator2`
                (`self.Electrocute` :!label _label_4))
              (:`NewEnumerator3`
                (`self.SlamOpen/Close` :!label _label_5))
              (:`NewEnumerator5`
                (`self.TriggerSpawn` :!label _label_6)))))
        (else
          (switch `/Game/Prototype/Blueprints/Enum_InteractionSource` (`self.InteractionSource`)
            (:`NewEnumerator0`
              (goto _label))))))
    (:`NewEnumerator1`
      (switch `/Game/Prototype/Blueprints/Enum_InteractionBehaviour` (`self.OverloadBehaviour`)
        (:`NewEnumerator0`
          (goto _label_2))
        (:`NewEnumerator1`
          (goto _label_3))
        (:`NewEnumerator2`
          (goto _label_4))
        (:`NewEnumerator3`
          (goto _label_5))
        (:`NewEnumerator5`
          (goto _label_6))))
    (:`NewEnumerator2`
      ;[1 1 1] Increase/decrease energy drain for boobytrap
      (if (`self.Boobytrapped`)
        (set `self.Boobytrapped` false)
        (else
          (set `self.Boobytrapped` true))))))

(event `self.ShowToolTip`
  (`self.StartHighlight`))

(event `self.HideToolTip`
  (`self.StopHighlight`))

(event `BindHighlight`
  (bind _controller (`self.Controller`))
  (add `/Game/Prototype/Blueprints/Player/BP_Controller.OnStartHighlight` _controller (delegate `StartHighlight`))
  (add `/Game/Prototype/Blueprints/Player/BP_Controller.OnStopHighlight` _controller (delegate `StopHighlight`)))

(event `StartHighlight`
  (bind _childmesh (`self.ChildMesh`))
  (switch `/Game/Prototype/Blueprints/Objects/Enum_OnboardingChecks` (`self.EnabledInteractions`)
    (:`NewEnumerator1`
      _)
    (:`NewEnumerator2`
      _))
  (`PrimitiveComponent.SetRenderCustomDepth` _childmesh true)
  (`PrimitiveComponent.SetCustomDepthStencilValue` _childmesh 1))

(event `StopHighlight`
  (`PrimitiveComponent.SetRenderCustomDepth` (`self.ChildMesh`) false))

(event `Distract`
  (bind _returnvalue (`self.K2_GetActorLocation`))
  (bind _walktodistraction (`self.WalkToDistraction`))
  (bind _outhits (`KismetSystemLibrary.SphereTraceMulti` :`Start` _returnvalue :`End` _returnvalue :`Radius` (`self.DistractionRadius`) :`TraceChannel` "TraceTypeQuery5" :`DrawDebugType` "Persistent"))
  (set `self.ClosestTargetDistance` 10000.0)
  (for _array_element _outhits
    (bind (_bblockinghit _binitialoverlap _time _distance _location _impactpoint _normal _impactnormal _physmat _hitactor) (`GameplayStatics.BreakHitResult` _array_element))
    (bind _returnvalue_2 (`KismetMathLibrary.Vector_Distance` _location (`self.K2_GetActorLocation` _hitactor)))
    (if (< _returnvalue_2 (`self.ClosestTargetDistance`))
      (set `self.ClosestTargetDistance` _returnvalue_2)
      (bind _asbp_third_person_character (cast `/Game/Prototype/Blueprints/Characters/BP_ThirdPersonCharacter` _hitactor))
      (set `self.DistractionTarget` _asbp_third_person_character)))
  (`GameplayStatics.PlaySoundAtLocation` (`self.Sound`) (`self.K2_GetActorLocation`) (struct) 1.0 1.0 0.0 null null null null)
  (`/Engine/EditorBlueprintResources/StandardMacros.IsValid` (`self.MoveToActor`)
    (:`Is Valid`
      (message `/Game/Prototype/Blueprints/BI_Character.Distract` (`self.DistractionTarget`) _walktodistraction (`self.K2_GetActorLocation`) (`self.MoveToActor`)))
    (:`Is Not Valid`
      (message `/Game/Prototype/Blueprints/BI_Character.Distract` (`self.DistractionTarget`) _walktodistraction (`self.K2_GetActorLocation`) self))))

(event `Electrocute`
  (bind _returnvalue (`self.K2_GetActorLocation`))
  (bind _outhits (`KismetSystemLibrary.SphereTraceMulti` _returnvalue _returnvalue (`self.ElectrocutionRadius`) "TraceTypeQuery5"))
  (for _array_element _outhits
    ;[1 1 1] Electrocute character(s)
    (message `/Game/Prototype/Blueprints/BI_Ragdoll.EnableRagdoll` (`.HitActor` (`GameplayStatics.BreakHitResult` _array_element)) (0.0 0.0 0.0))))

(event `Open/CLose`
  (`self.TriggerOpen/Close` 5.0))

(event `SlamOpen/Close`
  (`self.TriggerOpen/Close` 50.0))

(event `self.ReceiveTick`
  (params (DeltaSeconds :type "Float (single-precision)"))
  (bind _overloadbar (`self.OverloadBar`))
  (bind (_relativerotation_roll _relativerotation_pitch _relativerotation_yaw) (`KismetMathLibrary.BreakRotator` (`SceneComponent.RelativeRotation` (`self.MovableComponent`))))
  (if (`SceneComponent.bVisible` _overloadbar)
    (`SceneComponent.K2_SetWorldRotation` _overloadbar (`KismetMathLibrary.FindLookAtRotation` (`SceneComponent.K2_GetComponentLocation` _overloadbar) (`SceneComponent.K2_GetComponentLocation` (`Actor.RootComponent` (`/Game/Prototype/Blueprints/Player/BP_Controller.CurrentPOVPawn` (`self.Controller`))))) false false))
  (if (`self.MovableBehaviourUsed`)
    (if (`self.MovableStatusUpdated`)
      _
      (elif (== _relativerotation_yaw (`self.TargetRotation`))
        (if (== _relativerotation_yaw (`self.MaxRotation`))
          (set `self.MovableOpen` true)
          (else
            (set `self.MovableOpen` false)))
        (set `self.MovableStatusUpdated` true)))))

(event `TriggerSpawn`
  (if (`self.Repeat Spawn`)
    (bind _returnvalue (`KismetSystemLibrary.K2_SetTimerDelegate` (delegate `Spawn`) (/ (`self.Repeat Time`) (`self.Repeat Amount`)) true))
    (set `self.SpawnTimer` _returnvalue)
    (else
      (`self.Spawn`))))

(event `Spawn`
  (bind (_returnvalue_roll _returnvalue_pitch _returnvalue_yaw) (`KismetMathLibrary.BreakRotator` (`self.K2_GetActorRotation`)))
  (bind _mesharray (`self.MeshArray`))
  (if (`KismetArrayLibrary.Array_IsNotEmpty` _mesharray)
    (bind _output_get (set `self.CurrentSceneComponent` (`KismetArrayLibrary.Array_Random` _mesharray)))
    (bind _returnvalue (`|SpawnActorFromClass` (`self.Actor to Spawn`) (`KismetMathLibrary.MakeTransform` (`SceneComponent.K2_GetComponentLocation` _output_get) (`KismetMathLibrary.MakeRotator` _returnvalue_roll _returnvalue_pitch _returnvalue_yaw) (`self.GetActorScale3D`)) "Undefined" "MultiplyWithRoot" null null))
    (`KismetArrayLibrary.Array_RemoveItem` _mesharray _output_get)
    (`ActorComponent.K2_DestroyComponent` _output_get)
    (if (> (`self.Spawn Force`) 0.0)
      (message `/Game/Prototype/Blueprints/BI_Interactable.InteractStart` _returnvalue null "NewEnumerator0" "NewEnumerator2" 0.0))
    (if (`self.Repeat Spawn`)
      (`/Engine/EditorBlueprintResources/StandardMacros.IncrementInt` (`self.SpawnCounter`)
        (:`  `
          (if (>= (`self.SpawnCounter`) (`self.Repeat Amount`))
            (`KismetSystemLibrary.K2_ClearAndInvalidateTimerHandle` (`self.SpawnTimer`))
            (set `self.SpawnCounter` 0)))))))

(event `/Game/Prototype/Blueprints/BI_Interactable.ShowOutline`
  (`self.StartHighlight`))

(event `/Game/Prototype/Blueprints/BI_Interactable.HideOutline`
  (`self.StopHighlight`))

(event `/Game/Prototype/Blueprints/BI_Interactable.ShowOverloadBar`
  (switch `/Game/Prototype/Blueprints/Objects/Enum_OnboardingChecks` (`self.EnabledInteractions`)
    (:`NewEnumerator1`
      _)
    (:`NewEnumerator2`
      _))
  (`SceneComponent.SetVisibility` (`self.OverloadBar`) true false))

(event `/Game/Prototype/Blueprints/BI_Interactable.HideOverloadBar`
  (`SceneComponent.SetVisibility` (`self.OverloadBar`) false false))

(event `/Game/Prototype/Blueprints/BI_Interactable.EnableInteraction`
  (params (Type :type "/Game/Prototype/Blueprints/Objects/Enum_OnboardingChecks Enum" :default "NewEnumerator0"))
  (set `self.EnabledInteractions` Type))

(fn `GetActivityAnimations`
  (returns (AnimIn :type "AnimSequence Object Reference") (AnimOut :type "AnimSequence Object Reference"))
  (return null null))

(fn `GetForcedNextTask`
  (returns (ForcedNextTask :type "/Game/Developers/harshistalker/Proto/Core/Objects/BP_WorldObject_HTmp Object Reference"))
  (return null))

(fn `GetHoverText`
  (returns (InteractText :type String) (OverloadText :type String) (BoobytrapText :type String))
  (return "Press [E] to distract" "Press [Q] to electrocute" "Press [F] to boobytrap"))

(fn `GetWorkerDestination`
  (returns (Transform :type "Transform Structure"))
  (return))

(fn `Initialize`
  (params (DistractionRadius :type "Float (double-precision)") (Sound :type "SoundBase Object Reference") (InteractBehaviour :type "/Game/Prototype/Blueprints/Enum_InteractionBehaviour Enum" :default "NewEnumerator0") (OverloadBehaviour :type "/Game/Prototype/Blueprints/Enum_InteractionBehaviour Enum" :default "NewEnumerator0") (ChildMesh :type "StaticMeshComponent Object Reference") (MoveToActor :type "Actor Object Reference") (WalkToDistraction :type Boolean) (MovableDoors :type "SceneComponent Object Reference") (SpawnLocationComponent :type "SceneComponent Object Reference") (SpawnForce :type "Float (double-precision)") (ActorToSpawn :type "Actor Class Reference") (RepeatSpawn :type Boolean) (RepeatAmount :type Integer) (RepeatTime :type "Float (double-precision)"))
  ;[1 1 1] Update variables based on child's settings
  (set `self.DistractionRadius` DistractionRadius)
  (set `self.Sound` Sound)
  (bind _asbp_third_person_game_mode (cast `/Game/Prototype/ThirdPerson/Blueprints/BP_ThirdPersonGameMode` (`GameplayStatics.GetGameMode`))
    (:`then`
      (set `self.GameMode` _asbp_third_person_game_mode))
    (:`CastFailed`
      _))
  (bind _asbp_controller (cast `/Game/Prototype/Blueprints/Player/BP_Controller` (`GameplayStatics.GetPlayerController` 0)))
  (set `self.Controller` _asbp_controller)
  (set `self.InteractBehaviour` InteractBehaviour)
  (set `self.OverloadBehaviour` OverloadBehaviour)
  (`self.BindHighlight`)
  (set `self.ChildMesh` ChildMesh)
  (set `self.MoveToActor` MoveToActor)
  (set `self.WalkToDistraction` WalkToDistraction)
  (bind _output_get (set `self.MovableComponent` MovableDoors))
  (`/Game/Prototype/Blueprints/AC_Rotator.Initialize` (`self.AC_Rotator`) _output_get)
  (set `self.SpawnLocationComponent` SpawnLocationComponent)
  (set `self.Spawn Force` SpawnForce)
  (set `self.Actor to Spawn` ActorToSpawn)
  (set `self.Repeat Spawn` RepeatSpawn)
  (set `self.Repeat Amount` RepeatAmount)
  (set `self.Repeat Time` RepeatTime)
  (if (or (== (`self.InteractBehaviour`) 1) (== (`self.OverloadBehaviour`) 4))
    (set `self.MovableBehaviourUsed` true)))

(fn `IsInteractableThroughWalls`
  (returns (InteractableThroughWalls :type Boolean))
  (return false))

(fn `TriggerOpen/Close`
  (params (Speed :type "Float (double-precision)"))
  (if (not (`/Game/Prototype/Blueprints/AC_Rotator.Moving` (`self.AC_Rotator`)))
    (if (`self.MovableOpen`)
      (set `self.TargetRotation` 0.0)
      (set `self.StartingRotation` (.yaw (.rotation (`SceneComponent.GetRelativeTransform` (`self.MovableComponent`)))))
      (else
        (set `self.TargetRotation` (`self.MaxRotation`))
        (set `self.StartingRotation` 0.0)))
    (set `self.MovableStatusUpdated` false)
    (`/Game/Prototype/Blueprints/AC_Rotator.StartRotating` (`self.AC_Rotator`) Speed (`KismetMathLibrary.MakeRotator` 0.0 0.0 (`self.StartingRotation`)) (`KismetMathLibrary.MakeRotator` 0.0 0.0 (`self.TargetRotation`)))))

(fn `UserConstructionScript`)