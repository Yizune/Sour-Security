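; BP_Paper is a prototype paper prop that ragdolls actors it hits at speed.
; When the mesh's hit event fires with velocity above a threshold, it sends an EnableRagdoll message to the other actor, passing a scaled copy of that velocity plus an upward boost.
; An AddForce event applies a given vector as an impulse to the mesh, letting other code launch the paper.
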(event `self.SM_Prop_Paper_Lewd_Copy_01.OnComponentHit`
  (params (HitComponent :type "PrimitiveComponent Object Reference") (OtherActor :type "Actor Object Reference") (OtherComp :type "PrimitiveComponent Object Reference") (NormalImpulse :type "Vector Structure") (Hit :type "HitResult Structure (by ref)"))
  (bind _returnvalue (`SceneComponent.GetComponentVelocity` (`self.SM_Prop_Paper_Lewd_Copy_01`)))
  (if (> (`KismetMathLibrary.VSize` _returnvalue) 100.0)
    (message `/Game/Prototype/Blueprints/BI_Ragdoll.EnableRagdoll` OtherActor (+ (* _returnvalue 5.0) (0.0 0.0 1000.0)))))

(event `/Game/Prototype/Blueprints/BI_Force.AddForce`
  (params (ForceVector :type "Vector Structure"))
  (`PrimitiveComponent.AddImpulse` (`self.SM_Prop_Paper_Lewd_Copy_01`) ForceVector "None" false))

(fn `UserConstructionScript`)