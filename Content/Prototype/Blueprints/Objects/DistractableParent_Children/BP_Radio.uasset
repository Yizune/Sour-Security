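; BP_Radio is a distractable world object, a radio child of the DistractableParent family that plays background audio.
; On BeginPlay it calls the parent's Initialize with its distraction radius, interact and overload behaviours, and mesh.
; It then spawns an attenuated radio sound at its location and registers that sound, paired with itself, in the level's BP_SoundManager.
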(event `self.ReceiveBeginPlay`
  (`self.Initialize` 1000.0 null "NewEnumerator1" "NewEnumerator4" (`self.StaticMesh`))
  (bind _returnvalue (`GameplayStatics.SpawnSoundAtLocation` "/Game/SFX/Ambience/RadioBackground.RadioBackground" (`self.K2_GetActorLocation`) (struct) 1.0 1.0 0.0 "/Game/SFX/SoundAttenuationSettigns.SoundAttenuationSettigns" null))
  (bind _returnvalue_2 (`GameplayStatics.GetActorOfClass` "/Game/SFX/BP_SoundManager.BP_SoundManager_C"))
  (`KismetArrayLibrary.Array_Add` (`/Game/SFX/BP_SoundManager.SoundsStruct` _returnvalue_2) (make `/Game/SFX/Struct_Sounds` _returnvalue self)))

(fn `UserConstructionScript`
  (`parent.UserConstructionScript`))