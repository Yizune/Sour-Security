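; BP_Fridge is a distractable object, a fridge with a hinged door that can hurt coworkers when overloaded.
; On BeginPlay it initializes the distraction setup with its mesh and door hinge, then spawns a looping hum and registers it with BP_SoundManager.
; When a coworker overlaps its box during an Overload interaction while the rotator is moving, it sends ragdoll and harm messages, passing the door's forward vector to the ragdoll.
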(event `self.ReceiveBeginPlay`
  (`self.Initialize` 700.0 null "NewEnumerator0" "NewEnumerator3" (`self.StaticMesh`) null false (`self.DoorHinge`))
  (bind _returnvalue (`GameplayStatics.SpawnSoundAtLocation` "/Game/SFX/Ambience/FridgeLoop.FridgeLoop" (`self.K2_GetActorLocation`) (struct) 1.0 1.0 0.0 "/Game/SFX/SoundAttenuationSettigns.SoundAttenuationSettigns" null))
  (bind _returnvalue_2 (`GameplayStatics.GetActorOfClass` "/Game/SFX/BP_SoundManager.BP_SoundManager_C"))
  (`KismetArrayLibrary.Array_Add` (`/Game/SFX/BP_SoundManager.SoundsStruct` _returnvalue_2) (make `/Game/SFX/Struct_Sounds` _returnvalue self)))

(event `self.Box.OnComponentBeginOverlap`
  (params (OverlappedComponent :type "PrimitiveComponent Object Reference") (OtherActor :type "Actor Object Reference") (OtherComp :type "PrimitiveComponent Object Reference") (OtherBodyIndex :type Integer) (bFromSweep :type Boolean) (SweepResult :type "HitResult Structure (by ref)"))
  (bind _asbp_coworker (cast `/Game/Core/AI/FirstIteration/NPCs/BP_Coworker` OtherActor))
  (switch `/Game/Prototype/Blueprints/Enum_InteractionType` (`self.TypeOfInteraction`)
    (:`NewEnumerator1`
      (if (`/Game/Prototype/Blueprints/AC_Rotator.Moving` (`self.AC_Rotator`))
        (message `/Game/Prototype/Blueprints/BI_Ragdoll.EnableRagdoll` OtherActor (`SceneComponent.GetForwardVector` (`self.DoorHinge`)))
        (message `/Game/Core/AI/FirstIteration/Interfaces/BPI_CoworkerPawn.CauseHarm` _asbp_coworker "NewEnumerator3")))))

(fn `UserConstructionScript`
  (`parent.UserConstructionScript`))