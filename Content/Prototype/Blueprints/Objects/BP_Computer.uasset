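; Interactable computer prop that by default distracts characters when used and sets off a group of computers when overloaded.
; Interactions route by configured behaviour (distract, electrocute, open/close), and boobytrapped computers turn permitted NPC use into an overload.
; Distract sphere-traces for a character, plays a sound registered with BP_SoundManager and sends it a distraction.
; Overload re-triggers itself plus random other BP_Computers, their count scaled by overload force.
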(event `self.InteractStart`
  (params (TriggeringActor :type "Actor Object Reference") (TypeOfInteraction :type "/Game/Prototype/Blueprints/Enum_InteractionType Enum" :default "NewEnumerator0") (SourceOfInteraction :type "/Game/Prototype/Blueprints/Enum_InteractionSource Enum" :default "NewEnumerator1") (OverloadForce :type "Float (double-precision)"))
  (set `self.TypeOfInteraction` TypeOfInteraction)
  (set `self.InteractionSource` SourceOfInteraction)
  (set `self.OverloadForce` OverloadForce)
  (switch `/Game/Prototype/Blueprints/Enum_InteractionType` (`self.TypeOfInteraction`)
    (:`NewEnumerator0`
      (if (`self.Boobytrapped`)
        (switch `/Game/Prototype/Blueprints/Enum_InteractionSource` (`self.InteractionSource`)
          (:`NewEnumerator1`
            (if (`self.NPCCanInteract`)
              ;[1 1 1] Trigger overload if boobytrapped and character is interacting
              (message `/Game/Prototype/Blueprints/BI_Interactable.InteractStart` self null "NewEnumerator1" (`self.InteractionSource`) 0.0)))
          (:`NewEnumerator0`
            (switch `/Game/Prototype/Blueprints/Enum_InteractionBehaviour` (`self.InteractBehaviour`) :!label _label
              (:`NewEnumerator0`
                (`self.Open/CLose` :!label _label_2))
              (:`NewEnumerator1`
                (`self.Distract` :!label _label_3))
              (:`NewEnumerator2`
                (`self.Electrocute` :!label _label_4))
              (:`NewEnumerator3`
                (`self.SlamOpen/Close` :!label _label_5)))))
        (else
          (switch `/Game/Prototype/Blueprints/Enum_InteractionSource` (`self.InteractionSource`)
            (:`NewEnumerator1`
              (if (`self.NPCCanInteract`)
                (goto _label)))
            (:`NewEnumerator0`
              (goto _label))))))
    (:`NewEnumerator1`
      (switch `/Game/Prototype/Blueprints/Enum_InteractionBehaviour` (`self.OverloadBehaviour`)
        (:`NewEnumerator0`
          (goto _label_2))
        (:`NewEnumerator1`
          (goto _label_3))
        (:`NewEnumerator2`
          (goto _label_4))
        (:`NewEnumerator3`
          (goto _label_5))
        (:`NewEnumerator5`
          (`self.DistractMultiple`))))))

(event `BindHighlight`
  (bind _controller (`self.Controller`))
  (add `/Game/Prototype/Blueprints/Player/BP_Controller.OnStartHighlight` _controller (delegate `StartHighlight`))
  (add `/Game/Prototype/Blueprints/Player/BP_Controller.OnStopHighlight` _controller (delegate `StopHighlight`)))

(event `self.ShowOutline`
  (`self.StartHighlight`))

(event `StartHighlight`
  (`PrimitiveComponent.SetRenderCustomDepth` (`self.SM_Prop_Computer_Monitor_03`) true))

(event `StopHighlight`
  (`PrimitiveComponent.SetRenderCustomDepth` (`self.SM_Prop_Computer_Monitor_03`) false))

(event `self.HideOutline`
  (`self.StopHighlight`))

(event `Distract`
  (bind _returnvalue (`self.K2_GetActorLocation`))
  (bind _walktodistraction (`self.WalkToDistraction`))
  (bind _spawnedsound (`self.SpawnedSound`))
  (`/Engine/EditorBlueprintResources/StandardMacros.IsValid` _spawnedsound
    (:`Is Valid`
      (if (not (`AudioComponent.IsPlaying` _spawnedsound))
        (bind _outhits (`KismetSystemLibrary.SphereTraceMulti` :`Start` _returnvalue :`End` _returnvalue :`Radius` (`self.DistractionRadius`) :`TraceChannel` "TraceTypeQuery5" :`DrawDebugType` "Persistent" :!label _label_6))
        (set `self.ClosestTargetDistance` 10000.0)
        (for _array_element _outhits
          (bind (_bblockinghit _binitialoverlap _time _distance _location _impactpoint _normal _impactnormal _physmat _hitactor) (`GameplayStatics.BreakHitResult` _array_element))
          (bind _returnvalue_2 (`KismetMathLibrary.Vector_Distance` _location (`self.K2_GetActorLocation` _hitactor)))
          (if (< _returnvalue_2 (`self.ClosestTargetDistance`))
            (set `self.ClosestTargetDistance` _returnvalue_2)
            (bind _asbp_third_person_character (cast `/Game/Prototype/Blueprints/Characters/BP_ThirdPersonCharacter` _hitactor))
            (set `self.DistractionTarget` _asbp_third_person_character)))
        (bind _returnvalue_3 (`GameplayStatics.SpawnSoundAtLocation` (`self.Sound`) (`self.K2_GetActorLocation`) (struct) 1.0 1.0 0.0 "/Game/SFX/SoundAttenuationSettigns.SoundAttenuationSettigns" null false))
        (bind _returnvalue_4 (`GameplayStatics.GetActorOfClass` "/Game/SFX/BP_SoundManager.BP_SoundManager_C"))
        (`KismetArrayLibrary.Array_Add` (`/Game/SFX/BP_SoundManager.SoundsStruct` _returnvalue_4) (make `/Game/SFX/Struct_Sounds` _returnvalue_3 self))
        (set `self.SpawnedSound` null)
        (`SceneComponent.SetVisibility` (`self.Censor`) true false)
        (`/Engine/EditorBlueprintResources/StandardMacros.IsValid` (`self.MoveToActor`)
          (:`Is Valid`
            (message `/Game/Prototype/Blueprints/BI_Character.Distract` (`self.DistractionTarget`) _walktodistraction (`self.K2_GetActorLocation`) (`self.MoveToActor`)))
          (:`Is Not Valid`
            (message `/Game/Prototype/Blueprints/BI_Character.Distract` (`self.DistractionTarget`) _walktodistraction (`self.K2_GetActorLocation`) self)))))
    (:`Is Not Valid`
      (goto _label_6))))

(event `DistractMultiple`
  (bind _monitorstotrigger (`self.MonitorsToTrigger`))
  (bind _outitem (`KismetArrayLibrary.Array_Random` (`self.Monitors`)))
  (`KismetArrayLibrary.Array_Clear` _monitorstotrigger)
  (`KismetArrayLibrary.Array_Add` _monitorstotrigger self)
  (set `self.TriggerNumber` (+ (* (`KismetArrayLibrary.Array_Length` (`self.Monitors`)) (`self.OverloadForce`)) 1))
  (while (< (`KismetArrayLibrary.Array_Length` (`self.MonitorsToTrigger`)) (`self.TriggerNumber`))
    (if (== (`KismetArrayLibrary.Array_Find` (`self.MonitorsToTrigger`) _outitem) -1)
      (`KismetArrayLibrary.Array_Add` (`self.MonitorsToTrigger`) _outitem)))
  (for _array_element (`self.MonitorsToTrigger`)
    (message `/Game/Prototype/Blueprints/BI_Interactable.InteractStart` _array_element null "NewEnumerator0" "NewEnumerator0" 0.0)))

(event `Electrocute`
  (bind _returnvalue (`self.K2_GetActorLocation`))
  (bind _outhits (`KismetSystemLibrary.SphereTraceMulti` _returnvalue _returnvalue (`self.ElectrocutionRadius`) "TraceTypeQuery5"))
  (for _array_element _outhits
    (message `/Game/Prototype/Blueprints/BI_Ragdoll.EnableRagdoll` (`.HitActor` (`GameplayStatics.BreakHitResult` _array_element)) (0.0 0.0 0.0))))

(event `Open/CLose`
  (`self.TriggerOpen/Close` 5.0))

(event `SlamOpen/Close`
  (`self.TriggerOpen/Close` 12.5))

(event `self.ReceiveBeginPlay`
  (`self.Initialize` 750.0 "/Game/SFX/Objects/Computer/ComputerInteractionA.ComputerInteractionA" "NewEnumerator1" "NewEnumerator5"))

(event `self.ReceiveTick`
  (params (DeltaSeconds :type "Float (single-precision)"))
  (bind _overloadbar (`self.OverloadBar`))
  (if (`SceneComponent.bVisible` _overloadbar)
    (`SceneComponent.K2_SetWorldRotation` _overloadbar (`KismetMathLibrary.FindLookAtRotation` (`SceneComponent.K2_GetComponentLocation` _overloadbar) (`SceneComponent.K2_GetComponentLocation` (`Actor.RootComponent` (`/Game/Prototype/Blueprints/Player/BP_Controller.CurrentPOVPawn` (`self.Controller`))))) false false)))

(event `self.ShowOverloadBar`
  (switch `/Game/Prototype/Blueprints/Enum_InteractionBehaviour` (`self.OverloadBehaviour`)
    (:`NewEnumerator0`
      _)
    (:`NewEnumerator1`
      _)
    (:`NewEnumerator2`
      _)
    (:`NewEnumerator3`
      _)
    (:`NewEnumerator5`
      _))
  (`SceneComponent.SetVisibility` (`self.OverloadBar`) true false))

(event `self.HideOverloadBar`
  (switch `/Game/Prototype/Blueprints/Enum_InteractionBehaviour` (`self.OverloadBehaviour`)
    (:`NewEnumerator0`
      _)
    (:`NewEnumerator1`
      _)
    (:`NewEnumerator2`
      _)
    (:`NewEnumerator3`
      _)
    (:`NewEnumerator5`
      _))
  (`SceneComponent.SetVisibility` (`self.OverloadBar`) false false))

(fn `GetActivityAnimations`
  (returns (AnimIn :type "AnimSequence Object Reference") (AnimOut :type "AnimSequence Object Reference"))
  (return null null))

(fn `GetForcedNextTask`
  (returns (ForcedNextTask :type "/Game/Developers/harshistalker/Proto/Core/Objects/BP_WorldObject_HTmp Object Reference"))
  (return null))

(fn `GetHoverText`
  (returns (InteractText :type String) (OverloadText :type String) (BoobytrapText :type String))
  (return "Press [E] to distract" "Press [Q] to electrocute" "Press [F] to boobytrap"))

(fn `GetWorkerDestination`
  (returns (Transform :type "Transform Structure"))
  (return))

(fn `Initialize`
  (params (DistractionRadius :type "Float (double-precision)") (Sound :type "SoundBase Object Reference") (InteractBehaviour :type "/Game/Prototype/Blueprints/Enum_InteractionBehaviour Enum" :default "NewEnumerator0") (OverloadBehaviour :type "/Game/Prototype/Blueprints/Enum_InteractionBehaviour Enum" :default "NewEnumerator0") (ChildMesh :type "StaticMeshComponent Object Reference") (MoveToActor :type "Actor Object Reference") (WalkToDistraction :type Boolean) (MovableDoors :type "SceneComponent Object Reference") (SpawnLocationComponent :type "SceneComponent Object Reference") (SpawnForce :type "Float (double-precision)") (ActorToSpawn :type "Actor Class Reference") (RepeatSpawn :type Boolean) (RepeatAmount :type Integer) (RepeatTime :type "Float (double-precision)"))
  ;[1 1 1] Update variables based on child's settings
  (set `self.DistractionRadius` DistractionRadius)
  (set `self.Sound` Sound)
  (bind _asbp_third_person_game_mode (cast `/Game/Prototype/ThirdPerson/Blueprints/BP_ThirdPersonGameMode` (`GameplayStatics.GetGameMode`))
    (:`then`
      (set `self.GameMode` _asbp_third_person_game_mode))
    (:`CastFailed`
      _))
  (bind _asbp_controller (cast `/Game/Prototype/Blueprints/Player/BP_Controller` (`GameplayStatics.GetPlayerController` 0)))
  (set `self.Controller` _asbp_controller)
  (set `self.InteractBehaviour` InteractBehaviour)
  (set `self.OverloadBehaviour` OverloadBehaviour)
  (`self.BindHighlight`)
  (set `self.ChildMesh` ChildMesh)
  (set `self.MoveToActor` MoveToActor)
  (set `self.WalkToDistraction` WalkToDistraction)
  (bind _output_get (set `self.MovableComponent` MovableDoors))
  (`/Game/Prototype/Blueprints/AC_Rotator.Initialize` (`self.AC_Rotator`) _output_get)
  (set `self.SpawnLocationComponent` SpawnLocationComponent)
  (set `self.Spawn Force` SpawnForce)
  (set `self.Repeat Spawn` RepeatSpawn)
  (set `self.Repeat Amount` RepeatAmount)
  (set `self.Repeat Time` RepeatTime)
  (bind _returnvalue (`|CreateWidget` "/Game/UI/WB_OverloadBar.WB_OverloadBar_C"))
  (`WidgetComponent.SetWidget` (`self.OverloadBar`) _returnvalue)
  (bind _outactors (`GameplayStatics.GetAllActorsOfClass` "BP_Computer_C"))
  (bind _output_get_2 (set `self.Monitors` _outactors))
  (`KismetArrayLibrary.Array_RemoveItem` _output_get_2 self))

(fn `IsInteractableThroughWalls`
  (returns (InteractableThroughWalls :type Boolean))
  (return false))

(fn `TriggerOpen/Close`
  (params (Speed :type "Float (double-precision)"))
  (if (not (`/Game/Prototype/Blueprints/AC_Rotator.Moving` (`self.AC_Rotator`)))
    (if (`self.MovableOpen`)
      (set `self.TargetRotation` 0.0)
      (set `self.StartingRotation` (.yaw (.rotation (`SceneComponent.GetRelativeTransform` (`self.MovableComponent`)))))
      (else
        (set `self.TargetRotation` (`self.MaxRotation`))
        (set `self.StartingRotation` 0.0)))
    (set `self.MovableStatusUpdated` false)
    (`/Game/Prototype/Blueprints/AC_Rotator.StartRotating` (`self.AC_Rotator`) Speed (`KismetMathLibrary.MakeRotator` 0.0 0.0 (`self.StartingRotation`)) (`KismetMathLibrary.MakeRotator` 0.0 0.0 (`self.TargetRotation`)))))

(fn `UserConstructionScript`)