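; Patrol manager that spawns patrolling BP_ThirdPersonCharacter NPCs on BeginPlay and hands them marker routes.
; It sorts BP_PatrolMarkers into work and leisure pools, then spawns three NPCs on preset CaseLeisure routes.
; Further NPCs draw a random workspot plus leisure markers through DoN retries with occupancy checks, though each Random use re-rolls, so checked and assigned markers can differ.
; An unconnected branch for assigning existing NPCs to workspots never runs.
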(event `self.ReceiveBeginPlay`
  (bind _workingmarkers (`self.WorkingMarkers`))
  (bind _caseleisure1 (`self.CaseLeisure1`))
  (bind _caseleisure2 (`self.CaseLeisure2`))
  (bind _caseleisure3 (`self.CaseLeisure3`))
  (bind _outitem (`KismetArrayLibrary.Array_Random` _workingmarkers))
  (bind _outitem_2 (`KismetArrayLibrary.Array_Random` (`self.LeisureMarkers`)))
  (bind _outactors (`GameplayStatics.GetAllActorsOfClass` "/Game/Prototype/Blueprints/Characters/AI/BP_PatrolMarker.BP_PatrolMarker_C"))
  (for _array_element _outactors
    (switch `/Game/Prototype/Blueprints/Characters/AI/Enum_TypeOfLocation` (`/Game/Prototype/Blueprints/Characters/AI/BP_PatrolMarker.TypeOfLocation` _array_element)
      (:`NewEnumerator0`
        (`KismetArrayLibrary.Array_Add` (`self.WorkingMarkers`) _array_element))
      (:`NewEnumerator1`
        (`KismetArrayLibrary.Array_Add` (`self.LeisureMarkers`) _array_element))))
  (for _index (range 3)
    (bind _returnvalue (`|SpawnActorFromClass` "/Game/Prototype/Blueprints/Characters/BP_ThirdPersonCharacter.BP_ThirdPersonCharacter_C" (`KismetMathLibrary.MakeTransform` (0.0 0.0 0.0)) "Undefined" "MultiplyWithRoot" null null))
    (set `/Game/Prototype/Blueprints/Characters/BP_ThirdPersonCharacter.Patrol` true _returnvalue)
    (switch `int` _index
      (:`0`
        (`self.K2_SetActorLocation` _returnvalue (+ (`self.K2_GetActorLocation` (`|GetArrayItem` _caseleisure1)) (0.0 0.0 90.0)) false false)
        (set `/Game/Prototype/Blueprints/Characters/BP_ThirdPersonCharacter.PatrolMarkers` _caseleisure1 _returnvalue))
      (:`1`
        (`self.K2_SetActorLocation` _returnvalue (+ (`self.K2_GetActorLocation` (`|GetArrayItem` _caseleisure2)) (0.0 0.0 90.0)) false false)
        (set `/Game/Prototype/Blueprints/Characters/BP_ThirdPersonCharacter.PatrolMarkers` _caseleisure2 _returnvalue))
      (:`2`
        (`self.K2_SetActorLocation` _returnvalue (+ (`self.K2_GetActorLocation` (`|GetArrayItem` _caseleisure3)) (0.0 0.0 90.0)) false false)
        (set `/Game/Prototype/Blueprints/Characters/BP_ThirdPersonCharacter.PatrolMarkers` _caseleisure3 _returnvalue))))
  (for _ (range 11)
    (bind _returnvalue_2 (`|SpawnActorFromClass` "/Game/Prototype/Blueprints/Characters/BP_ThirdPersonCharacter.BP_ThirdPersonCharacter_C" (`KismetMathLibrary.MakeTransform` (0.0 0.0 0.0)) "Undefined" "MultiplyWithRoot" null null))
    (set `/Game/Prototype/Blueprints/Characters/BP_ThirdPersonCharacter.Patrol` true _returnvalue_2)
    (bind _patrolmarkers (`/Game/Prototype/Blueprints/Characters/BP_ThirdPersonCharacter.PatrolMarkers` _returnvalue_2))
    (`KismetArrayLibrary.Array_Add` _patrolmarkers _outitem)
    (`self.K2_SetActorLocation` _returnvalue_2 (+ (`self.K2_GetActorLocation` _outitem) (0.0 0.0 90.0)) false false)
    (`KismetArrayLibrary.Array_RemoveItem` _workingmarkers _outitem)
    (`/Engine/EditorBlueprintResources/StandardMacros.Do N` 100 :!label _label
      (:`Exit`
        (if (< (`KismetArrayLibrary.Array_Length` (`/Game/Prototype/Blueprints/Characters/AI/BP_PatrolMarker.AssignedNPCs` _outitem_2)) 3)
          (if (== (`KismetArrayLibrary.Array_Find` _patrolmarkers _outitem_2) -1)
            (`KismetArrayLibrary.Array_Add` _patrolmarkers _outitem_2)
            (`KismetArrayLibrary.Array_Add` (`/Game/Prototype/Blueprints/Characters/AI/BP_PatrolMarker.AssignedNPCs` _outitem_2))
            (`|ExecutionSequence`
              (:`then_0`
                (goto _label :!via `Reset`))
              (:`then_1`
                (if (not (> (`KismetArrayLibrary.Array_Length` _patrolmarkers) 3))
                  (goto _label))))
            (else
              (goto _label)))
          (else
            (goto _label)))))))

(fn `UserConstructionScript`)