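; BP_TargetsManager tracks elimination targets across three stages and drives progression to the win screen.
; EliminationCheck saves the coworker's mesh location as its reset point, removes it from CurrentTargets and calls NextArea once that list empties.
; NextArea swaps in the next target set and enables its objects through BP_OnboardingManager, finally showing WBP_Win.
; SpareCheck calls GameOver for coworkers meant to be spared, but GameOver, GameWon and UpdateTargetState are stubs.
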(event `self.ReceiveBeginPlay`
  (set `self.CurrentTargets` (`self.Targets1`))
  (bind _returnvalue (`GameplayStatics.GetActorOfClass` "/Game/Prototype/Blueprints/Objects/OnBoarding/BP_OnboardingManager.BP_OnboardingManager_C"))
  (set `self.OnboardingManager` _returnvalue)
  (bind _asbp_controller (cast `/Game/Prototype/Blueprints/Player/BP_Controller` (`GameplayStatics.GetPlayerController` 0)))
  (set `self.BP Controller` _asbp_controller))

(event `SpareCheck`
  (params (CoworkerToCheck :type "/Game/Core/AI/FirstIteration/NPCs/BP_Coworker Object Reference"))
  (if (not (== (`KismetArrayLibrary.Array_Find` (`self.CoworkersToSpare`) CoworkerToCheck) -1))
    (`self.GameOver`)))

(event `EliminationCheck`
  (params (EliminatedCoworker :type "/Game/Core/AI/FirstIteration/NPCs/BP_Coworker Object Reference"))
  (bind _currenttargets (`self.CurrentTargets`))
  (bind _relativelocation (`SceneComponent.RelativeLocation` (`Character.Mesh` EliminatedCoworker)))
  (set `/Game/Core/AI/FirstIteration/NPCs/BP_Coworker.BackupReset` _relativelocation EliminatedCoworker)
  (set `/Game/Core/AI/FirstIteration/NPCs/BP_Coworker.ResetLocation` _relativelocation EliminatedCoworker)
  (`KismetArrayLibrary.Array_RemoveItem` _currenttargets EliminatedCoworker)
  (if (`KismetArrayLibrary.Array_IsEmpty` _currenttargets)
    (`/Engine/EditorBlueprintResources/StandardMacros.IncrementInt` (`self.TargetsIndex`)
      (:`  `
        (`self.NextArea`)))
    (else
      (`KismetSystemLibrary.PrintString` "targets left"))))

(event `NextArea`
  (bind _onboardingmanager (`self.OnboardingManager`))
  (switch `int` (`self.TargetsIndex`)
    (:`1`
      (set `self.CurrentTargets` (`self.Targets2`))
      (`/Game/Prototype/Blueprints/Objects/OnBoarding/BP_OnboardingManager.EnableObjects2` _onboardingmanager false false true))
    (:`2`
      (set `self.CurrentTargets` (`self.Targets3`))
      (`/Game/Prototype/Blueprints/Objects/OnBoarding/BP_OnboardingManager.EnableObjects3` _onboardingmanager false false true))
    (:`3`
      (`self.GameWon`)
      (bind _returnvalue (`|CreateWidget` "/Game/UI/WBP_Win.WBP_Win_C"))
      (`UserWidget.AddToViewport` _returnvalue 0))))

(event `GameOver`)

(event `UpdateTargetState`
  (params (Target :type "/Game/Core/AI/FirstIteration/NPCs/BP_Coworker Object Reference"))
  (for _ (`self.CurrentTargets`)
    _))

(event `GameWon`)

(fn `UserConstructionScript`)