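; BP_ObjectsCollection is a placed volume that switches the interaction state of every object inside it as a group.
; Its cube mesh is hidden shortly after BeginPlay.
; EnableObjects runs a multi box trace sized from the actor's scale at its location, then sends EnableInteractionMessage to each hit actor, with the enum value chosen by the Disable flag.
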(event `self.ReceiveBeginPlay`
  (`KismetSystemLibrary.Delay` 0.2)
  (`SceneComponent.SetVisibility` (`self.Cube`) false false))

(event `EnableObjects`
  (params (Disable :type Boolean))
  (bind _returnvalue (`self.K2_GetActorLocation`))
  (bind _returnvalue_2 (`self.K2_GetActorLocation`))
  (if Disable
    (bind _outhits (`KismetSystemLibrary.BoxTraceMulti` _returnvalue_2 _returnvalue_2 (* (`self.GetActorScale3D`) 50.0) (struct) "TraceTypeQuery3"))
    (for _array_element _outhits
      (message `/Game/Prototype/Blueprints/BI_Interactable.EnableInteraction` (`.HitActor` (`GameplayStatics.BreakHitResult` _array_element)) "NewEnumerator0"))
    (else
      (bind _outhits_2 (`KismetSystemLibrary.BoxTraceMulti` _returnvalue _returnvalue (* (`self.GetActorScale3D`) 50.0) (struct) "TraceTypeQuery3"))
      (for _array_element_2 _outhits_2
        (message `/Game/Prototype/Blueprints/BI_Interactable.EnableInteraction` (`.HitActor` (`GameplayStatics.BreakHitResult` _array_element_2)) "NewEnumerator2")))))

(fn `UserConstructionScript`)