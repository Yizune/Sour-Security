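; BI_Interactable is the Blueprint Interface for objects that can be interacted with, including overload and boobytrap hover text.
; It declares start and stop interaction calls, carrying the triggering actor, interaction type, source and an overload force.
; Feedback hooks cover outlines, blinking, the overload bar and hover text.
; Further functions expose activity animations, worker destination, forced next task, through-wall interactability, interaction enabling and a shift toggle.
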(fn `EnableInteraction`
  (params (Type :type "/Game/Prototype/Blueprints/Objects/Enum_OnboardingChecks Enum" :default "NewEnumerator0")))

(fn `GetActivityAnimations`
  (returns (AnimIn :type "AnimSequence Object Reference") (AnimOut :type "AnimSequence Object Reference"))
  (return null null))

(fn `GetForcedNextTask`
  (returns (ForcedNextTask :type "/Game/Developers/harshistalker/Proto/Core/Objects/BP_WorldObject_HTmp Object Reference"))
  (return null))

(fn `GetHoverText`
  (returns (InteractText :type String) (OverloadText :type String) (BoobytrapText :type String))
  (return "" "" ""))

(fn `GetWorkerDestination`
  (returns (Transform :type "Transform Structure"))
  (return))

(fn `HideOutline`)

(fn `HideOverloadBar`)

(fn `InteractStart`
  (params (TriggeringActor :type "Actor Object Reference") (TypeOfInteraction :type "/Game/Prototype/Blueprints/Enum_InteractionType Enum" :default "NewEnumerator0") (SourceOfInteraction :type "/Game/Prototype/Blueprints/Enum_InteractionSource Enum" :default "NewEnumerator0") (OverloadForce :type "Float (double-precision)"))
  (return))

(fn `InteractStop`)

(fn `IsInteractableThroughWalls`
  (returns (InteractableThroughWalls :type Boolean))
  (return false))

(fn `ShiftFunction`
  (params (Enable :type Boolean)))

(fn `ShowOutline`)

(fn `ShowOverloadBar`)

(fn `TriggerBlink`
  (params (Type :type "/Game/Prototype/Blueprints/Objects/Enum_OnboardingChecks Enum" :default "NewEnumerator0") (Index :type Integer)))